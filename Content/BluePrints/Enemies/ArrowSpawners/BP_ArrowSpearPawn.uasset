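; Spear pawn, launched along a spline by a timeline, that the snowball player can latch onto and steer.
; When the player hits the tip while holding Space, its capsule attaches to the hit cube and the spear takes possession and camera, registering with the spawner.
; Move inputs pitch the hit cube within limits based on the snap angle.
; Space release, through a DoOnce, or detachPlayer restores player physics and possession.
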(event OnComponentHit(hit_cube_collision)
  (params (HitComponent :type Primitive%20Component%20Object%20Reference) (OtherActor :type Actor%20Object%20Reference) (OtherComp :type Primitive%20Component%20Object%20Reference) (NormalImpulse :type Vector :default "0, 0, 0") (Hit :type Hit%20Result%20Structure%20%28by%20ref%29))
  (bind _hit_cube_collision (Variables|Components|Gethit_cube_collision))
  (bind _relativerotation (Variables|/Script/Engine.SceneComponent|GetRelativeRotation _hit_cube_collision))
  ;[1 1 1] The snowball hit the spear extremity
  (bind _asbp_player_paw (Utilities|Casting|CastToBP_PlayerPaw OtherActor))
  (Development|PrintString (Utilities|String|ToString(Float) (Math|Vector|DotProduct (.ImpactNormal (Collision|BreakHitResult Hit)) "0.000000,0.000000,1.000000")) true true "(R=0.000000,G=0.660000,B=1.000000,A=1.000000)" 1e+01)
  (if (Variables|/Game/BluePrints/Player/BP_PlayerPaw.BP_PlayerPaw_C|GetisSpaceHold _asbp_player_paw)
    (Physics|SetSimulatePhysics (Variables|/Game/BluePrints/Player/BP_PlayerPaw.BP_PlayerPaw_C|GetCapsule _asbp_player_paw) false)
    (Transformation|AttachComponentToComponent (Variables|/Game/BluePrints/Player/BP_PlayerPaw.BP_PlayerPaw_C|GetCapsule _asbp_player_paw) (Variables|Components|Gethit_cube_collision) "SomeSocket" "KeepWorld" "KeepWorld" "KeepWorld" true)
    (bind _output_get (Variables|Default|SetisSnap true))
    (Variables|/Game/BluePrints/Player/BP_PlayerPaw.BP_PlayerPaw_C|SetisSnap _asbp_player_paw _output_get)
    (Variables|/Game/BluePrints/Enemies/ArrowSpawners/BP_ArrowsSpawner.BP_ArrowsSpawner_C|SetarrowSnapedRef (Variables|Default|GetArrowSpawnerRef) (Variables|Default|GetArrowRef))
    (Variables|Default|SetRotationWhenSnapped (+ (.pitch _relativerotation) -9e+01))
    (Variables|Default|SetrelRotHitCube (.pitch _relativerotation))
    (Development|PrintString (Utilities|String|ToString(Float) (.pitch _relativerotation)) true true "(R=1.000000,G=0.601638,B=0.000000,A=1.000000)")
    (bind _asbp_player_controller (Utilities|Casting|CastToBP_PlayerController (Game|GetPlayerController 0)))
    (Pawn|Possess _asbp_player_controller self)
    (Game|Player|SetViewTargetwithBlend _asbp_player_controller self 0.0 "VTBlend_Linear" 0.0 false)))

(event Custom|detachPlayer
  (params (ArrowSnapedRef :type Name))
  ;[1 1 1] Forcément là puisque c'est ici que les contrôles ont lieu!
  (bind _returnvalue (Actor|GetActorOfClass "/Game/BluePrints/Player/BP_PlayerPaw.BP_PlayerPaw_C"))
  (Variables|Default|SetisSnap false)
  (Default|ResetSpaceHold _returnvalue)
  (Development|PrintString "space bar pressed")
  (Transformation|DetachFromComponent (Variables|/Game/BluePrints/Player/BP_PlayerPaw.BP_PlayerPaw_C|GetCapsule _returnvalue) "KeepWorld" "KeepWorld" "KeepWorld" true)
  (Transformation|SetWorldLocation (Variables|/Game/BluePrints/Player/BP_PlayerPaw.BP_PlayerPaw_C|GetCapsule _returnvalue) (Math|Vector|MakeVector (.x (Transformation|GetWorldLocation (Variables|/Game/BluePrints/Player/BP_PlayerPaw.BP_PlayerPaw_C|GetCapsule _returnvalue))) 0.0 (.z (Transformation|GetWorldLocation (Variables|/Game/BluePrints/Player/BP_PlayerPaw.BP_PlayerPaw_C|GetCapsule _returnvalue)))) false false)
  (bind _returnvalue_2 (Actor|GetActorOfClass "/Game/BluePrints/Player/BP_PlayerController.BP_PlayerController_C"))
  (Pawn|Possess _returnvalue_2 _returnvalue)
  (Physics|SetSimulatePhysics (Variables|/Game/BluePrints/Player/BP_PlayerPaw.BP_PlayerPaw_C|GetCapsule _returnvalue) true)
  (Transformation|SetRelativeRotation (Variables|Components|Gethit_cube_collision) "0, 0, 0" false false)
  (Utilities|FlowControl|DoOnce false) ; enters at Reset
)

(event Custom|LaunchArrow
  (bind _arrowsplineref (Variables|Default|GetArrowSplineRef))
  ;[1 1 1] Move component between two points described by distance between them
  (Variables|Default|SetArrowRef (Utilities|String|StringToName (Utilities|GetObjectName self)))
  (Variables|Default|SetSimpleStartPoint (Variables|/Script/Engine.SceneComponent|GetRelativeLocation (Variables|Components|Getbox)))
  (Components|Timeline|SetPlayRate (Variables|Default|GetMovingTimeline) (Variables|Default|GetPATROL_RATE))
  (bind _newtrack_0 (Timeline|MovingTimeline PlayFromStart)
    (:Update
      (Transformation|SetRelativeLocation (Variables|Components|Getbox) (Math|Vector|MakeVector (* (.x (Spline|GetLocationatDistanceAlongSpline _arrowsplineref (Math|Float|Lerp 0.0 (Spline|GetSplineLength _arrowsplineref) _newtrack_0) "Local")) (Variables|Default|GetIS_REVERSED_SIGN)) 0.0 (* (Variables|Default|GetIS_REVERSED_SIGN) (.z (Spline|GetLocationatDistanceAlongSpline _arrowsplineref (Math|Float|Lerp 0.0 (Spline|GetSplineLength _arrowsplineref) _newtrack_0) "Local")))) false false))))

(event Input|EnhancedActionEvents|EnhancedInputActionBP_Free
  (params (ActionValue :type Boolean) (ElapsedSeconds :type Float%20%28double-precision%29) (TriggeredSeconds :type Float%20%28double-precision%29) (InputAction :type Input%20Action%20Object%20Reference :default "/Game/BluePrints/Player/inputs/BP_Free.BP_Free")))

(event Input|EnhancedActionEvents|EnhancedInputActionBP_Move
  (params (ActionValue :type Vector :default "0, 0, 0") (ElapsedSeconds :type Float%20%28double-precision%29) (TriggeredSeconds :type Float%20%28double-precision%29) (InputAction :type Input%20Action%20Object%20Reference :default "/Game/BluePrints/Player/inputs/BP_Move.BP_Move"))
  (bind _rotationwhensnapped (Variables|Default|GetRotationWhenSnapped))
  ;[1 1 1] rotate hit cube attached between two angles
  (:Triggered
    (if (Variables|Default|GetisSnap) :!label _label
      (if (or (and (>= (+ (Variables|Default|GetrelRotHitCube) 1.5 0.0) (+ _rotationwhensnapped -45.0)) (<= (+ (Variables|Default|GetrelRotHitCube) 1.5 0.0) 0.0)) (and (<= (+ (Variables|Default|GetrelRotHitCube) 1.5 0.0) (+ _rotationwhensnapped 45.0)) (>= (+ (Variables|Default|GetrelRotHitCube) 1.5 0.0) 0.0)))
        (Variables|Default|SetrelRotHitCube (+ (Variables|Default|GetrelRotHitCube) 1.5 0.0))
        (Development|PrintString (Utilities|String|ToString(Float) (+ (Variables|Default|GetrelRotHitCube) 1.5 0.0)))
        (Transformation|SetRelativeRotation (Variables|Components|Gethit_cube_collision) (Math|Rotator|MakeRotator 0.0 (Variables|Default|GetrelRotHitCube) 0.0) false false))))
  (:Started
    (goto _label))
  (:Ongoing
    (goto _label)))

(event Input|EnhancedActionEvents|EnhancedInputActionBP_RightMove
  (params (ActionValue :type Vector :default "0, 0, 0") (ElapsedSeconds :type Float%20%28double-precision%29) (TriggeredSeconds :type Float%20%28double-precision%29) (InputAction :type Input%20Action%20Object%20Reference :default "/Game/BluePrints/Player/inputs/BP_RightMove.BP_RightMove"))
  (bind _rotationwhensnapped (Variables|Default|GetRotationWhenSnapped))
  ;[1 1 1] rotate hit cube attached between two angles
  (:Triggered
    (if (Variables|Default|GetisSnap) :!label _label
      (if (or (and (>= (+ (Variables|Default|GetrelRotHitCube) -1.5 0.0) (+ _rotationwhensnapped -45.0)) (<= (+ (Variables|Default|GetrelRotHitCube) -1.5 0.0) 0.0)) (and (<= (+ (Variables|Default|GetrelRotHitCube) -1.5 0.0) (+ _rotationwhensnapped 45.0)) (>= (+ (Variables|Default|GetrelRotHitCube) -1.5 0.0) 0.0)))
        (Variables|Default|SetrelRotHitCube (+ (Variables|Default|GetrelRotHitCube) -1.5 0.0))
        (Development|PrintString (Utilities|String|ToString(Float) (+ (Variables|Default|GetrelRotHitCube) -1.5 0.0)))
        (Transformation|SetRelativeRotation (Variables|Components|Gethit_cube_collision) (Math|Rotator|MakeRotator 0.0 (Variables|Default|GetrelRotHitCube) 0.0) false false))))
  (:Started
    (goto _label))
  (:Ongoing
    (goto _label)))

(event EventTick
  (params (DeltaSeconds :type Float%20%28single-precision%29)))

(event Input|KeyboardEvents|SpaceBar
  (params (Key :type Key%20Structure))
  ;[1 1 1] Forcément là puisque c'est ici que les contrôles ont lieu!
  (:Released
    (Utilities|FlowControl|DoOnce false :!label _label
      (:Completed
        (bind _returnvalue (Actor|GetActorOfClass "/Game/BluePrints/Player/BP_PlayerPaw.BP_PlayerPaw_C"))
        (Variables|Default|SetisSnap false)
        (Default|ResetSpaceHold _returnvalue)
        (Development|PrintString "space bar pressed")
        (Transformation|DetachFromComponent (Variables|/Game/BluePrints/Player/BP_PlayerPaw.BP_PlayerPaw_C|GetCapsule _returnvalue) "KeepWorld" "KeepWorld" "KeepWorld" true)
        (Transformation|SetWorldLocation (Variables|/Game/BluePrints/Player/BP_PlayerPaw.BP_PlayerPaw_C|GetCapsule _returnvalue) (Math|Vector|MakeVector (.x (Transformation|GetWorldLocation (Variables|/Game/BluePrints/Player/BP_PlayerPaw.BP_PlayerPaw_C|GetCapsule _returnvalue))) 0.0 (.z (Transformation|GetWorldLocation (Variables|/Game/BluePrints/Player/BP_PlayerPaw.BP_PlayerPaw_C|GetCapsule _returnvalue)))) false false)
        (bind _returnvalue_2 (Actor|GetActorOfClass "/Game/BluePrints/Player/BP_PlayerController.BP_PlayerController_C"))
        (Pawn|Possess _returnvalue_2 _returnvalue)
        (Physics|SetSimulatePhysics (Variables|/Game/BluePrints/Player/BP_PlayerPaw.BP_PlayerPaw_C|GetCapsule _returnvalue) true)
        (Transformation|SetRelativeRotation (Variables|Components|Gethit_cube_collision) "0, 0, 0" false false)
        (goto _label Reset)))))

(fn ConstructionScript)