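; BP_ArrowsSpawner is an enemy arrow spawner that repeatedly fires BP_ArrowSpearPawn arrows from the start of its spline.
; A BeginPlay delay loop spawns each arrow, passes it the spawner, spline and speed, then launches it.
; When the spawner's yaw exceeds a near-180 threshold, it reverses the arrow's sign and box.
; An end-point overlap destroys arriving arrows, first detaching the player if the arrow is snapped.
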(event OnComponentBeginOverlap(endarrowpoint)
  (params (OverlappedComponent :type Primitive%20Component%20Object%20Reference) (OtherActor :type Actor%20Object%20Reference) (OtherComp :type Primitive%20Component%20Object%20Reference) (OtherBodyIndex :type Integer) (bFromSweep :type Boolean) (SweepResult :type Hit%20Result%20Structure%20%28by%20ref%29))
  (bind _asbp_arrow_spear_pawn (Utilities|Casting|CastToBP_ArrowSpearPawn OtherActor))
  (if (Variables|/Game/BluePrints/Enemies/ArrowSpawners/BP_ArrowSpearPawn.BP_ArrowSpearPawn_C|GetisSnap _asbp_arrow_spear_pawn)
    (Default|DetachPlayer _asbp_arrow_spear_pawn (Variables|Default|GetarrowSnapedRef)))
  (Actor|DestroyActor _asbp_arrow_spear_pawn))

(event EventBeginPlay
  (bind _returnvalue (Game|SpawnActorfromClass "/Game/BluePrints/Enemies/ArrowSpawners/BP_ArrowSpearPawn.BP_ArrowSpearPawn_C" (Math|Transform|MakeTransform (Class|SplineComponent|GetLocationatSplineInputKey (Variables|Default|GetArrowSpline) 0.0 "World") "0, 0, 0" "1.000000,1.000000,1.000000") "Undefined" "MultiplyWithRoot" 0 0 :!label _label))
  (Variables|/Game/BluePrints/Enemies/ArrowSpawners/BP_ArrowSpearPawn.BP_ArrowSpearPawn_C|SetArrowSpawnerRef _returnvalue self)
  (Variables|/Game/BluePrints/Enemies/ArrowSpawners/BP_ArrowSpearPawn.BP_ArrowSpearPawn_C|SetArrowSplineRef _returnvalue (Variables|Default|GetArrowSpline))
  (Variables|/Game/BluePrints/Enemies/ArrowSpawners/BP_ArrowSpearPawn.BP_ArrowSpearPawn_C|SetPATROL_RATE _returnvalue (Variables|Default|GetarrowSpeedRate))
  (if (> (.yaw (Transformation|GetWorldRotation (Variables|Default|GetDefaultSceneRoot))) 179.0)
    (Variables|/Game/BluePrints/Enemies/ArrowSpawners/BP_ArrowSpearPawn.BP_ArrowSpearPawn_C|SetIS_REVERSED_SIGN _returnvalue -1)
    (Transformation|SetRelativeRotation (Variables|/Game/BluePrints/Enemies/ArrowSpawners/BP_ArrowSpearPawn.BP_ArrowSpearPawn_C|Getbox _returnvalue) (Math|Rotator|MakeRotator 0.0 0.0 1.8e+02) false false))
  (Default|LaunchArrow _returnvalue)
  (Utilities|FlowControl|Delay (Variables|Default|GetspawnDelay))
  (goto _label))

(event Collision|EventActorBeginOverlap
  (params (OtherActor :type Actor%20Object%20Reference)))

(event EventTick
  (params (DeltaSeconds :type Float%20%28single-precision%29)))

(fn ConstructionScript)