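; Boss-fight trigger volume that hands the camera to the boss camera when the player pawn overlaps its Cube.
; The first overlap blends the view target to the BP_BossCamera in the level, closes the BP_SimpleMovingDoor named "Gate7", then destroys the trigger.
; A DoOnce, reset on end overlap, gates a FlipFlop whose second branch returns the view to the player, though self-destruction on the first pass leaves it effectively unused.
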(event OnComponentBeginOverlap(Cube)
  (params (OverlappedComponent :type Primitive%20Component%20Object%20Reference) (OtherActor :type Actor%20Object%20Reference) (OtherComp :type Primitive%20Component%20Object%20Reference) (OtherBodyIndex :type Integer) (bFromSweep :type Boolean) (SweepResult :type Hit%20Result%20Structure%20%28by%20ref%29))
  (bind _asbp_player_paw (Utilities|Casting|CastToBP_PlayerPaw OtherActor))
  (Utilities|FlowControl|DoOnce false
    (:Completed
      (Utilities|FlowControl|FlipFlop
        (:A
          (bind _returnvalue (Actor|GetActorOfClass "/Game/BluePrints/Enemies/BOSS/BP_BossCamera.BP_BossCamera_C"))
          (Game|Player|SetViewTargetwithBlend (Game|GetPlayerController 0) _returnvalue 0.0 "VTBlend_Linear" 0.0 false)
          (bind _outactors (Actor|GetAllActorsOfClass "/Game/BluePrints/Immobiles/BP_SimpleMovingDoor.BP_SimpleMovingDoor_C"))
          (bind _array_element (Utilities|Array|ForEachLoopwithBreak _outactors :!label _label)
            (:LoopBody
              (if (Utilities|Enum|Equal(Enum) (Variables|/Game/BluePrints/Immobiles/BP_SimpleMovingDoor.BP_SimpleMovingDoor_C|GetGateNameString _array_element) "Gate7")
                (Default|CloseGate _array_element)
                (goto _label Break)))
            (:Completed
              (Actor|DestroyActor))))
        (:B
          (Game|Player|SetViewTargetwithBlend (Game|GetPlayerController 0) _asbp_player_paw 0.0 "VTBlend_Linear" 0.0 false))))))

(event OnComponentEndOverlap(Cube)
  (params (OverlappedComponent :type Primitive%20Component%20Object%20Reference) (OtherActor :type Actor%20Object%20Reference) (OtherComp :type Primitive%20Component%20Object%20Reference) (OtherBodyIndex :type Integer))
  (Utilities|FlowControl|DoOnce false) ; enters at Reset
)

(event EventBeginPlay)

(event Collision|EventActorBeginOverlap
  (params (OtherActor :type Actor%20Object%20Reference)))

(event EventTick
  (params (DeltaSeconds :type Float%20%28single-precision%29)))

(fn ConstructionScript)