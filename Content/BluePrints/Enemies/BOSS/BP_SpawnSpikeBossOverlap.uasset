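; Boss attack trigger that, when activated and overlapped by the player, rains a timed series of spikes at the player's position.
; Overlap clears IsActivated and starts a self-recalling, delay-paced loop, stopped after a few seconds through IsLooping, which then re-arms.
; Each pass samples the player's X before a short delay, then spawns a rotated BP_Spike at fixed height, applies its Saint material and triggers its move-then-destroy sequence.
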(event Custom|SpawnLoopSpikeAtPlayerLocation
  (params (PlayerRef :type BP%20Player%20Paw%20Object%20Reference))
  (if (Variables|Default|GetisLooping)
    (bind _output_get (Variables|Default|SetpreviousPlayerX (.x (Transformation|GetWorldLocation (Variables|/Game/BluePrints/Player/BP_PlayerPaw.BP_PlayerPaw_C|GetCapsule PlayerRef)))))
    (Utilities|FlowControl|Delay 0.5)
    (bind _returnvalue (Game|SpawnActorfromClass "/Game/BluePrints/Immobiles/BP_Spike.BP_Spike_C" (Math|Transform|MakeTransform (Math|Vector|MakeVector _output_get 0.0 1041.0) "0.000000,180.000000,180.000000" "1.000000,1.000000,1.000000") "Undefined" "MultiplyWithRoot" 0 0))
    (Default|ChangeMaterialtoSaint _returnvalue)
    (Default|MovefromtheGroundThenDestroy _returnvalue)
    (Utilities|FlowControl|Delay 0.6)
    (CallFunction|SpawnLoopSpikeatPlayerLocation PlayerRef)
    (else
      (Utilities|FlowControl|Delay 0.2)
      (Variables|Default|SetisLooping true))))

(event EventBeginPlay)

(event Collision|EventActorBeginOverlap
  (params (OtherActor :type Actor%20Object%20Reference))
  (if (Variables|Default|GetisActivated)
    (bind _asbp_player_paw (Utilities|Casting|CastToBP_PlayerPaw OtherActor))
    (Development|PrintString "TREBOBOSS")
    (Variables|Default|SetisActivated false)
    (CallFunction|SpawnLoopSpikeatPlayerLocation _asbp_player_paw)
    (Utilities|FlowControl|Delay 4.0)
    (Variables|Default|SetisLooping false)))

(event EventTick
  (params (DeltaSeconds :type Float%20%28single-precision%29)))

(fn ConstructionScript)