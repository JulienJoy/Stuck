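; Spear-wielding 2D enemy that patrols along a spline and doubles as a perch the player can latch onto.
; Timelines chained by FlipFlops cycle spear thrusts, head rotation and patrol moves, with flags toggling each stage.
; Hitting the spear's hit cube while holding Space attaches the player pawn and possesses the enemy, optionally starting its patrol.
; Move inputs then tilt the cube within limits, and releasing Space detaches and repossesses the pawn.
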(event OnComponentHit(hit_cube_collision)
  (params (HitComponent :type Primitive%20Component%20Object%20Reference) (OtherActor :type Actor%20Object%20Reference) (OtherComp :type Primitive%20Component%20Object%20Reference) (NormalImpulse :type Vector :default "0, 0, 0") (Hit :type Hit%20Result%20Structure%20%28by%20ref%29))
  ;[1 1 1] The snowball hit the spear extremity
  (bind _asbp_player_paw (Utilities|Casting|CastToBP_PlayerPaw OtherActor))
  (Development|PrintString (Utilities|String|ToString(Float) (Math|Vector|DotProduct (.ImpactNormal (Collision|BreakHitResult Hit)) "0.000000,0.000000,1.000000")) true true "(R=0.000000,G=0.660000,B=1.000000,A=1.000000)" 1e+01)
  (if (Variables|/Game/BluePrints/Player/BP_PlayerPaw.BP_PlayerPaw_C|GetisSpaceHold _asbp_player_paw)
    (Physics|SetSimulatePhysics (Variables|/Game/BluePrints/Player/BP_PlayerPaw.BP_PlayerPaw_C|GetCapsule _asbp_player_paw) false)
    (Transformation|AttachComponentToComponent (Variables|/Game/BluePrints/Player/BP_PlayerPaw.BP_PlayerPaw_C|GetCapsule _asbp_player_paw) (Variables|Components|Gethit_cube_collision) "SomeSocket" "KeepWorld" "KeepWorld" "KeepWorld" true)
    (bind _output_get (Variables|Default|SetisSnap true))
    (Variables|/Game/BluePrints/Player/BP_PlayerPaw.BP_PlayerPaw_C|SetisSnap _asbp_player_paw _output_get)
    (Development|PrintString (Utilities|String|ToString(Float) (.pitch (Variables|/Script/Engine.SceneComponent|GetRelativeRotation (Variables|Components|Gethit_cube_collision)))) true true "(R=1.000000,G=0.601638,B=0.000000,A=1.000000)")
    (bind _asbp_player_controller (Utilities|Casting|CastToBP_PlayerController (Game|GetPlayerController 0)))
    (Pawn|Possess _asbp_player_controller self)
    (Game|Player|SetViewTargetwithBlend _asbp_player_controller self 1e+01 "VTBlend_EaseInOut" 1.0 false)
    (if (Variables|Basicbehavior|GetIS_MOVING_WHEN_PLAYER)
      (Utilities|FlowControl|DoOnce false
        (:Completed
          (Variables|Basicbehavior|SetIS_ENEMY_MOVING true)
          (CallFunction|MoveAlongDefinedSpline))))))

(event Custom|inverseSpriteSign
  (bind _enemy_sprite_backward (Variables|Default|GetENEMY_SPRITE_BACKWARD))
  (bind _enemypapersprite (Variables|Default|GetEnemyPaperSprite))
  (bind _enemy_sprite_forward (Variables|Default|GetENEMY_SPRITE_FORWARD))
  (if (== (Variables|Default|Getcurrent_ENEMY_SPRITE) (Variables|Default|GetENEMY_SPRITE_FORWARD))
    (Rendering|Components|Sprite|SetSprite _enemypapersprite _enemy_sprite_backward)
    (Variables|Default|Setcurrent_ENEMY_SPRITE _enemy_sprite_backward)
    (else
      (Rendering|Components|Sprite|SetSprite _enemypapersprite _enemy_sprite_forward)
      (Variables|Default|Setcurrent_ENEMY_SPRITE _enemy_sprite_forward))))

(event Custom|Move%20Along%20Defined%20Spline
  ;[1 1 1] Move component between two points described by distance between them
  (if (Variables|Basicbehavior|GetIS_ENEMY_MOVING)
    (Variables|Default|Setcurrent_ENEMY_SPRITE (Variables|Default|GetENEMY_SPRITE_BACKWARD))
    (CallFunction|InverseSpriteSign)
    (Components|Timeline|SetPlayRate (Variables|Default|Getmoving%20AlongSpline%20Timeline) (Variables|Basicbehavior|GetPATROL_RATE))
    (bind _newtrack_0 (Timeline|moving%20AlongSpline%20Timeline PlayFromStart)
      (:Update
        (Transformation|SetRelativeLocation (Variables|Components|Getbox) (Math|Vector|MakeVector (.x (Spline|GetLocationatDistanceAlongSpline (Variables|Default|GetTrajectorySpline) (Math|Float|Lerp 0.0 (Spline|GetSplineLength (Variables|Default|GetTrajectorySpline)) _newtrack_0) "Local")) 0.0 (.z (Spline|GetLocationatDistanceAlongSpline (Variables|Default|GetTrajectorySpline) (Math|Float|Lerp 0.0 (Spline|GetSplineLength (Variables|Default|GetTrajectorySpline)) _newtrack_0) "Local"))) false false))
      (:Finished
        (CallFunction|MoveSpearUpThenDown :!label _label)))
    (else
      (goto _label))))

(event Custom|moveSpearUpThenDown
  (bind _hit_cube_collision (Variables|Components|Gethit_cube_collision))
  (bind _spear1 (Variables|Components|Getspear1))
  (Rendering|Components|Sprite|SetSprite (Variables|Default|GetEnemyPaperSprite) "/Game/BluePrints/Enemies/enemyMageIdle_Sprite.enemyMageIdle_Sprite")
  ;[1 1 1] move spear up THEN down
  (if (Variables|Basicbehavior|GetIS_MOVE_SPEAR)
    (Variables|Default|SetHitCubeIdleRelativeLocation (Variables|/Script/Engine.SceneComponent|GetRelativeLocation _hit_cube_collision))
    (Variables|Default|SetSpearIdleRelativeLocation (Variables|/Script/Engine.SceneComponent|GetRelativeLocation _spear1))
    (bind _spearuptrack (Timeline|moving%20Spear%20Timeline PlayFromStart)
      (:Update
        (Transformation|SetRelativeLocation _hit_cube_collision (Math|Vector|MakeVector 0.0 0.0 (+ (.z (Variables|Default|GetHitCubeIdleRelativeLocation)) (Math|Float|Lerp 0.0 (Variables|Basicbehavior|GetSPEAR_POWER) _spearuptrack))) false false)
        (Transformation|SetRelativeLocation _spear1 (Math|Vector|MakeVector 0.0 0.0 (+ (.z (Variables|Default|GetSpearIdleRelativeLocation)) (Math|Float|Lerp 0.0 (Variables|Basicbehavior|GetSPEAR_POWER) _spearuptrack))) false false))
      (:Finished
        (Utilities|FlowControl|FlipFlop
          (:A
            (Utilities|FlowControl|Delay (Variables|Basicbehavior|GetTIME_BETWEEN_SPEAR_SWITCH))
            (Timeline|moving%20Spear%20Timeline ReverseFromEnd))
          (:B
            (Utilities|FlowControl|FlipFlop :!label _label
              (:A
                (CallFunction|RotateUpSpear))
              (:B
                (CallFunction|RotateDownSpear)))))))
    (else
      (Utilities|FlowControl|Delay (Variables|Basicbehavior|GetTIME_BETWEEN_SPEAR_ROTATE))
      (goto _label))))

(event Custom|rotateUpSpear
  ;[1 1 1] rotate head so spear ON  AND OFF
  (Variables|Basicbehavior|SetSPEAR_POWER (Variables|SpearMoveConstraint|GetNORMAL_SPEAR_POWER))
  (Variables|SpearMoveConstraint|SetSpearPhase "NewEnumerator0")
  (if (Variables|SpearMoveConstraint|GetisCanSpearPhaseA)
    _
    (else
      (Variables|Basicbehavior|SetSPEAR_POWER 0.0)))
  (if (Variables|Basicbehavior|GetIS_ROTATE_SPEAR)
    (bind _newtrack_0 (Timeline|rotate%20Timeline PlayFromStart)
      (:Update
        (Transformation|SetRelativeRotation (Variables|Default|Gethead) (Math|Rotator|MakeRotator 0.0 (Math|Float|Lerp 0.0 (Variables|Basicbehavior|GetROTATION_ANGLE_Y) _newtrack_0) 0.0) false false))
      (:Finished
        (Utilities|FlowControl|FlipFlop
          (:A
            (CallFunction|MoveSpearUpThenDown))
          (:B
            (CallFunction|ReturntoIdlePosition :!label _label)))))
    (else
      (goto _label))))

(event Custom|rotateDownSpear
  ;[1 1 1] rotate head so spear ON  AND OFF
  (Variables|Basicbehavior|SetSPEAR_POWER (Variables|SpearMoveConstraint|GetNORMAL_SPEAR_POWER))
  (Variables|SpearMoveConstraint|SetSpearPhase "NewEnumerator1")
  (if (Variables|SpearMoveConstraint|GetisCanSpearPhaseB)
    _
    (else
      (Variables|Basicbehavior|SetSPEAR_POWER 0.0)))
  (if (Variables|Basicbehavior|GetIS_ROTATE_SPEAR)
    (bind _newtrack_0 (Timeline|rotate%20Timeline ReverseFromEnd)
      (:Update
        (Transformation|SetRelativeRotation (Variables|Default|Gethead) (Math|Rotator|MakeRotator 0.0 (Math|Float|Lerp 0.0 (Variables|Basicbehavior|GetROTATION_ANGLE_Y) _newtrack_0) 0.0) false false))
      (:Finished
        (Utilities|FlowControl|FlipFlop
          (:A
            (CallFunction|MoveSpearUpThenDown))
          (:B
            (CallFunction|ReturntoIdlePosition :!label _label)))))
    (else
      (goto _label))))

(event Custom|returnToIdlePosition
  ;[1 1 1] Move component between two points described by distance between them
  (if (Variables|Basicbehavior|GetIS_ENEMY_MOVING)
    (CallFunction|InverseSpriteSign)
    (Utilities|FlowControl|FlipFlop
      (:A
        (bind _newtrack_0 (Timeline|moving%20AlongSpline%20Timeline ReverseFromEnd)
          (:Update
            (Transformation|SetRelativeLocation (Variables|Components|Getbox) (Math|Vector|MakeVector (.x (Spline|GetLocationatDistanceAlongSpline (Variables|Default|GetTrajectorySpline) (Math|Float|Lerp 0.0 (Spline|GetSplineLength (Variables|Default|GetTrajectorySpline)) _newtrack_0) "Local")) 0.0 (.z (Spline|GetLocationatDistanceAlongSpline (Variables|Default|GetTrajectorySpline) (Math|Float|Lerp 0.0 (Spline|GetSplineLength (Variables|Default|GetTrajectorySpline)) _newtrack_0) "Local"))) false false))
          (:Finished
            (CallFunction|MoveSpearUpThenDown :!label _label))))
      (:B
        (Timeline|moving%20AlongSpline%20Timeline PlayFromStart)))
    (else
      (goto _label))))

(event Input|EnhancedActionEvents|EnhancedInputActionBP_Free
  (params (ActionValue :type Boolean) (ElapsedSeconds :type Float%20%28double-precision%29) (TriggeredSeconds :type Float%20%28double-precision%29) (InputAction :type Input%20Action%20Object%20Reference :default "/Game/BluePrints/Player/inputs/BP_Free.BP_Free")))

(event Input|EnhancedActionEvents|EnhancedInputActionBP_Move
  (params (ActionValue :type Vector :default "0, 0, 0") (ElapsedSeconds :type Float%20%28double-precision%29) (TriggeredSeconds :type Float%20%28double-precision%29) (InputAction :type Input%20Action%20Object%20Reference :default "/Game/BluePrints/Player/inputs/BP_Move.BP_Move"))
  ;[1 1 1] rotate hit cube attached between two angles
  (:Triggered
    (if (Variables|Default|GetisSnap) :!label _label
      (if (or (and (>= (+ (Variables|Default|GetrelRotHitCube) 1.5 0.0) (+ 0.0 -45.0)) (<= (+ (Variables|Default|GetrelRotHitCube) 1.5 0.0) 0.0)) (and (<= (+ (Variables|Default|GetrelRotHitCube) 1.5 0.0) (+ 0.0 45.0)) (>= (+ (Variables|Default|GetrelRotHitCube) 1.5 0.0) 0.0)))
        (Variables|Default|SetrelRotHitCube (+ (Variables|Default|GetrelRotHitCube) 1.5 0.0))
        (Development|PrintString (Utilities|String|ToString(Float) (+ (Variables|Default|GetrelRotHitCube) 1.5 0.0)))
        (Transformation|SetRelativeRotation (Variables|Components|Gethit_cube_collision) (Math|Rotator|MakeRotator 0.0 (Variables|Default|GetrelRotHitCube) 0.0) false false))))
  (:Started
    (goto _label))
  (:Ongoing
    (goto _label)))

(event Input|EnhancedActionEvents|EnhancedInputActionBP_RightMove
  (params (ActionValue :type Vector :default "0, 0, 0") (ElapsedSeconds :type Float%20%28double-precision%29) (TriggeredSeconds :type Float%20%28double-precision%29) (InputAction :type Input%20Action%20Object%20Reference :default "/Game/BluePrints/Player/inputs/BP_RightMove.BP_RightMove"))
  ;[1 1 1] rotate hit cube attached between two angles
  (:Triggered
    (if (Variables|Default|GetisSnap) :!label _label
      (if (or (and (>= (+ (Variables|Default|GetrelRotHitCube) -1.5 0.0) (+ 0.0 -45.0)) (<= (+ (Variables|Default|GetrelRotHitCube) -1.5 0.0) 0.0)) (and (<= (+ (Variables|Default|GetrelRotHitCube) -1.5 0.0) (+ 0.0 45.0)) (>= (+ (Variables|Default|GetrelRotHitCube) -1.5 0.0) 0.0)))
        (Variables|Default|SetrelRotHitCube (+ (Variables|Default|GetrelRotHitCube) -1.5 0.0))
        (Development|PrintString (Utilities|String|ToString(Float) (+ (Variables|Default|GetrelRotHitCube) -1.5 0.0)))
        (Transformation|SetRelativeRotation (Variables|Components|Gethit_cube_collision) (Math|Rotator|MakeRotator 0.0 (Variables|Default|GetrelRotHitCube) 0.0) false false))))
  (:Started
    (goto _label))
  (:Ongoing
    (goto _label)))

(event EventBeginPlay
  (bind _trajectoryspline (Variables|Default|GetTrajectorySpline))
  (bind _returnvalue (Spline|GetArriveTangentatSplinePoint _trajectoryspline 1 "Local"))
  (bind _returnvalue_2 (/ (.z _returnvalue) (.x _returnvalue)))
  (bind _returnvalue_3 (Class|KismetMathLibrary|DegAtan _returnvalue_2))
  (Variables|SpearMoveConstraint|SetNORMAL_SPEAR_POWER (Variables|Basicbehavior|GetSPEAR_POWER))
  (if (Variables|SpearMoveConstraint|GetisCanSpearPhaseB)
    _
    (else
      (Variables|Basicbehavior|SetSPEAR_POWER 0.0)))
  (Development|PrintString (Utilities|String|ToString(Float) _returnvalue_3))
  (if (>= _returnvalue_3 0.0)
    (Variables|Default|SetENEMY_SPRITE_FORWARD "/Game/BluePrints/Enemies/enemyMageMoving_Sprite.enemyMageMoving_Sprite")
    ;[1 1 1] begin to move "patrol"
    (Variables|Default|SetENEMY_SPRITE_BACKWARD "/Game/BluePrints/Enemies/enemyMageMovingInverted_Sprite.enemyMageMovingInverted_Sprite")
    (else
      (Variables|Default|SetENEMY_SPRITE_FORWARD "/Game/BluePrints/Enemies/enemyMageMovingInverted_Sprite.enemyMageMovingInverted_Sprite")
      (Variables|Default|SetENEMY_SPRITE_BACKWARD "/Game/BluePrints/Enemies/enemyMageMoving_Sprite.enemyMageMoving_Sprite")))
  (if (not (Variables|Basicbehavior|GetIS_MOVING_WHEN_PLAYER))
    (CallFunction|MoveAlongDefinedSpline)))

(event Input|KeyboardEvents|SpaceBar
  (params (Key :type Key%20Structure))
  ;[1 1 1] Forcément là puisque c'est ici que les contrôles ont lieu!
  (:Released
    (Utilities|FlowControl|DoOnce false :!label _label
      (:Completed
        (bind _returnvalue (Actor|GetActorOfClass "/Game/BluePrints/Player/BP_PlayerPaw.BP_PlayerPaw_C"))
        (Default|ResetSpaceHold _returnvalue)
        (Development|PrintString "space bar pressed")
        (Transformation|DetachFromComponent (Variables|/Game/BluePrints/Player/BP_PlayerPaw.BP_PlayerPaw_C|GetCapsule _returnvalue) "KeepWorld" "KeepWorld" "KeepWorld" true)
        (Transformation|SetWorldLocation (Variables|/Game/BluePrints/Player/BP_PlayerPaw.BP_PlayerPaw_C|GetCapsule _returnvalue) (Math|Vector|MakeVector (.x (Transformation|GetWorldLocation (Variables|/Game/BluePrints/Player/BP_PlayerPaw.BP_PlayerPaw_C|GetCapsule _returnvalue))) 0.0 (.z (Transformation|GetWorldLocation (Variables|/Game/BluePrints/Player/BP_PlayerPaw.BP_PlayerPaw_C|GetCapsule _returnvalue)))) false false)
        (bind _returnvalue_2 (Actor|GetActorOfClass "/Game/BluePrints/Player/BP_PlayerController.BP_PlayerController_C"))
        (Pawn|Possess _returnvalue_2 _returnvalue)
        (Physics|SetSimulatePhysics (Variables|/Game/BluePrints/Player/BP_PlayerPaw.BP_PlayerPaw_C|GetCapsule _returnvalue) true)
        (Transformation|SetRelativeRotation (Variables|Components|Gethit_cube_collision) "0, 0, 0" false false)
        (goto _label Reset)))))

(fn ConstructionScript
  (if (Variables|Basicbehavior|GetIS_ENEMY_MOVING)
    _
    (else
      _))
  (Transformation|SetWorldLocation (Variables|Default|GetCube) (Class|SplineComponent|GetLocationatSplineInputKey (Variables|Default|GetTrajectorySpline) 1.0 "World") false false))

(fn ConstraintPhase
  (params (SpearPhaseToConstraint :type BPE_AttackAouB%20Enum :default "NewEnumerator0"))
  (if (Variables|SpearMoveConstraint|GetisCanSpearPhaseA)
    (Variables|Basicbehavior|SetSPEAR_POWER 0.0)))