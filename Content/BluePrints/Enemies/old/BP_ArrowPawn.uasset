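; Enemy arrow (spear) pawn that flies a set distance along X on a Timeline, then destroys itself, releasing any snapped player.
; If the player snowball hits the tip while holding Space, its capsule attaches to the hit cube and the controller possesses this pawn.
; While snapped, move inputs pitch the cube in clamped steps.
; Releasing Space detaches and re-possesses the player, with BP_CameraFollow as view target throughout.
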(event OnComponentHit(hit_cube_collision)
  (params (HitComponent :type Primitive%20Component%20Object%20Reference) (OtherActor :type Actor%20Object%20Reference) (OtherComp :type Primitive%20Component%20Object%20Reference) (NormalImpulse :type Vector :default "0, 0, 0") (Hit :type Hit%20Result%20Structure%20%28by%20ref%29))
  (bind (_bblockinghit _binitialoverlap _time _distance _location _impactpoint _normal _impactnormal) (Collision|BreakHitResult Hit))
  (bind _hit_cube_collision (Variables|Components|Gethit_cube_collision))
  (bind (_x _y _z) (Math|Vector|BreakVector _impactpoint))
  (bind _returnvalue (* _impactnormal "-100.000000,-100.000000,-100.000000"))
  (bind _returnvalue_2 (+ _impactpoint _returnvalue))
  (bind (_x_2 _y_2 _z_2) (Math|Vector|BreakVector _returnvalue_2))
  ;[1 1 1] The snowball hit the spear extremity
  (bind _asbp_player_paw (Utilities|Casting|CastToBP_PlayerPaw OtherActor))
  (if (Variables|/Game/BluePrints/Player/BP_PlayerPaw.BP_PlayerPaw_C|GetisSpaceHold _asbp_player_paw)
    (bind _output_get (Variables|Default|SetanotherVector (Math|Vector|MakeVector (- _x_2 _x) (- _y_2 _y) (- _z_2 _z))))
    (Collision|LineTraceByChannel _impactpoint _returnvalue_2 "TraceTypeQuery1" false 0 "ForDuration" true "(R=1.000000,G=0.000000,B=0.000000,A=1.000000)" "(R=0.000000,G=1.000000,B=0.000000,A=1.000000)" 1e+01)
    (Utilities|FlowControl|DoOnce false
      (:Completed
        (Development|PrintString (Utilities|String|Append "Player hit enemy spear " (Utilities|String|ToString(Vector) _impactnormal) "  pitch : " (Utilities|String|ToString(Float) (.Pitch (Math|Vector|GetYawPitchfromVector _output_get)))) true true "(R=0.000000,G=0.660000,B=1.000000,A=1.000000)" 12.0)
        (Variables|Default|SetrectificationAngle (.Pitch (Math|Vector|GetYawPitchfromVector _output_get)))
        (Variables|/Game/BluePrints/Player/BP_PlayerPaw.BP_PlayerPaw_C|SetanchoredComponent _asbp_player_paw _hit_cube_collision)
        (Variables|Default|SetisSnap true)
        (Variables|/Game/BluePrints/Player/BP_PlayerPaw.BP_PlayerPaw_C|SetisSnap _asbp_player_paw true)
        (Variables|Components|SetattachedComponent (Variables|/Game/BluePrints/Player/BP_PlayerPaw.BP_PlayerPaw_C|GetCapsule _asbp_player_paw))
        (Transformation|AttachComponentToComponent (Variables|/Game/BluePrints/Player/BP_PlayerPaw.BP_PlayerPaw_C|GetCapsule _asbp_player_paw) _hit_cube_collision "SomeSocket" "KeepWorld" "KeepWorld" "KeepWorld" true)
        (Physics|SetSimulatePhysics (Variables|Components|Gethit_cube_collision) false)
        (bind _asbp_player_controller (Utilities|Casting|CastToBP_PlayerController (Game|GetPlayerController 0)))
        (Pawn|Possess _asbp_player_controller self)
        (Development|PrintString (Utilities|String|ToString(Float) (.pitch (Transformation|GetWorldRotation (Variables|/Game/BluePrints/Player/BP_PlayerPaw.BP_PlayerPaw_C|GetCapsule _asbp_player_paw)))) true true "(R=1.000000,G=0.179992,B=0.000000,A=1.000000)" 1e+01)
        (bind _returnvalue_3 (Actor|GetActorOfClass "/Game/BluePrints/Player/BP_CameraFollow.BP_CameraFollow_C"))
        (Game|Player|SetViewTargetwithBlend _asbp_player_controller _returnvalue_3 0.0 "VTBlend_Linear" 0.0 false)))))

(event Custom|detachPlayer
  ;[1 1 1] Forcément là puisque c'est ici que les contrôles ont lieu!
  (Development|PrintString "player datched")
  (bind _returnvalue (Actor|GetActorOfClass "/Game/BluePrints/Player/BP_PlayerPaw.BP_PlayerPaw_C"))
  (Default|ResetSpaceHold _returnvalue)
  (Development|PrintString "space bar pressed")
  (Transformation|DetachFromComponent (Variables|/Game/BluePrints/Player/BP_PlayerPaw.BP_PlayerPaw_C|GetCapsule _returnvalue) "KeepWorld" "KeepWorld" "KeepWorld" true)
  (Physics|SetSimulatePhysics (Variables|Components|Gethit_cube_collision) false)
  (bind _returnvalue_2 (Actor|GetActorOfClass "/Game/BluePrints/Player/BP_PlayerController.BP_PlayerController_C"))
  (Pawn|Possess _returnvalue_2 _returnvalue)
  (bind _returnvalue_3 (Actor|GetActorOfClass "/Game/BluePrints/Player/BP_CameraFollow.BP_CameraFollow_C"))
  (Game|Player|SetViewTargetwithBlend _returnvalue_2 _returnvalue_3 0.0 "VTBlend_Linear" 0.0 false))

(event Custom|launchArrow
  (bind _box2 (Variables|Components|GetBox2))
  (bind _hit_cube_collision (Variables|Components|Gethit_cube_collision))
  (bind _defaultsceneroot (Variables|Components|GetDefaultSceneRoot))
  (bind _enemydistancepatrol (Variables|Default|GetenemyDistancePatrol))
  (bind _returnvalue (Transformation|GetWorldLocation _defaultsceneroot))
  (bind _relativelocation (Variables|/Script/Engine.SceneComponent|GetRelativeLocation _box2))
  ;[1 1 1] Move component between two points described by distance between them
  (bind _output_get (Variables|Default|SetstartLocationX (.x _returnvalue)))
  (Variables|Default|SetrelLocHitCube (Math|Vector|MakeVector (.x _relativelocation) (.y _relativelocation) (.z _relativelocation)))
  (Components|Timeline|SetPlayRate (Variables|Default|GetTimeline) (Variables|Default|GetpatrolRate))
  (bind _newtrack_0 (Timeline|Timeline PlayFromStart)
    (:Update
      (Transformation|SetWorldLocation _defaultsceneroot (Math|Vector|MakeVector (+ _output_get (* _newtrack_0 (Variables|Default|GetenemyDistancePatrol))) 0.0 (.z _returnvalue)) false false)
      (Transformation|SetWorldLocation _box2 (Math|Vector|MakeVector (+ (+ _output_get (* _newtrack_0 (Variables|Default|GetenemyDistancePatrol))) (* (/ _enemydistancepatrol (Math|Float|Absolute(Float) _enemydistancepatrol)) 77.0)) 0.0 (.z (Transformation|GetWorldLocation _box2))) false false)
      (Transformation|SetWorldLocation _hit_cube_collision (Math|Vector|MakeVector (+ (+ _output_get (* _newtrack_0 (Variables|Default|GetenemyDistancePatrol))) (* (/ _enemydistancepatrol (Math|Float|Absolute(Float) _enemydistancepatrol)) 77.0)) 0.0 (.z (Transformation|GetWorldLocation _hit_cube_collision))) false false))
    (:Finished
      (Variables|Default|Settick true))))

(event Input|EnhancedActionEvents|EnhancedInputActionBP_Move
  (params (ActionValue :type Vector :default "0, 0, 0") (ElapsedSeconds :type Float%20%28double-precision%29) (TriggeredSeconds :type Float%20%28double-precision%29) (InputAction :type Input%20Action%20Object%20Reference :default "/Game/BluePrints/Player/inputs/BP_Move.BP_Move"))
  (bind _hit_cube_collision (Variables|Components|Gethit_cube_collision))
  (bind _returnvalue (Transformation|GetWorldRotation _hit_cube_collision))
  (bind _returnvalue_2 (+ (.pitch _returnvalue) 5.0 0.0))
  ;[1 1 1] rotate hit cube attached between two angles
  (:Triggered
    (if (Variables|Default|GetisSnap) :!label _label
      (Development|PrintString (Utilities|String|ToString(Float) _returnvalue_2))
      (if (or (and (>= _returnvalue_2 (+ 0.0 -9e+01)) (<= _returnvalue_2 0.0)) (and (<= _returnvalue_2 (+ 0.0 9e+01)) (>= _returnvalue_2 0.0)))
        (Transformation|SetWorldRotation _hit_cube_collision (Math|Rotator|MakeRotator 0.0 _returnvalue_2 0.0) false false))))
  (:Started
    (goto _label))
  (:Ongoing
    (goto _label)))

(event Input|EnhancedActionEvents|EnhancedInputActionBP_RightMove
  (params (ActionValue :type Vector :default "0, 0, 0") (ElapsedSeconds :type Float%20%28double-precision%29) (TriggeredSeconds :type Float%20%28double-precision%29) (InputAction :type Input%20Action%20Object%20Reference :default "/Game/BluePrints/Player/inputs/BP_RightMove.BP_RightMove"))
  (bind _hit_cube_collision (Variables|Components|Gethit_cube_collision))
  (bind _returnvalue (Transformation|GetWorldRotation _hit_cube_collision))
  (bind _returnvalue_2 (+ (.pitch _returnvalue) -5.0 0.0))
  ;[1 1 1] rotate hit cube attached between two angles
  (:Triggered
    (if (Variables|Default|GetisSnap) :!label _label
      (Development|PrintString (Utilities|String|ToString(Float) _returnvalue_2))
      (if (or (and (>= _returnvalue_2 (+ 0.0 -9e+01)) (<= _returnvalue_2 0.0)) (and (<= _returnvalue_2 (+ 0.0 9e+01)) (>= _returnvalue_2 0.0)))
        (Transformation|SetWorldRotation _hit_cube_collision (Math|Rotator|MakeRotator 0.0 _returnvalue_2 0.0) false false))))
  (:Started
    (goto _label))
  (:Ongoing
    (goto _label)))

(event EventBeginPlay
  ;[1 1 1] Move component between two points described by distance between them
)

(event EventTick
  (params (DeltaSeconds :type Float%20%28single-precision%29))
  (bind _enemydistancepatrol (Variables|Default|GetenemyDistancePatrol))
  (if (Variables|Default|Gettick)
    (if (== (.x (Transformation|GetWorldLocation (Variables|Components|GetBox2))) (+ (+ (Variables|Default|GetstartLocationX) _enemydistancepatrol) (* (/ _enemydistancepatrol (Math|Float|Absolute(Float) _enemydistancepatrol)) 77.0)))
      (if (Variables|Default|GetisSnap)
        (CallFunction|DetachPlayer))
      (Actor|DestroyActor))))

(event Input|KeyboardEvents|SpaceBar
  (params (Key :type Key%20Structure))
  ;[1 1 1] Forcément là puisque c'est ici que les contrôles ont lieu!
  (:Released
    (Utilities|FlowControl|DoOnce false
      (:Completed
        (bind _returnvalue (Actor|GetActorOfClass "/Game/BluePrints/Player/BP_PlayerPaw.BP_PlayerPaw_C"))
        (Default|ResetSpaceHold _returnvalue)
        (Development|PrintString "space bar pressed")
        (Transformation|DetachFromComponent (Variables|/Game/BluePrints/Player/BP_PlayerPaw.BP_PlayerPaw_C|GetCapsule _returnvalue) "KeepWorld" "KeepWorld" "KeepWorld" true)
        (Physics|SetSimulatePhysics (Variables|Components|Gethit_cube_collision) false)
        (bind _returnvalue_2 (Actor|GetActorOfClass "/Game/BluePrints/Player/BP_PlayerController.BP_PlayerController_C"))
        (Pawn|Possess _returnvalue_2 _returnvalue)
        (bind _returnvalue_3 (Actor|GetActorOfClass "/Game/BluePrints/Player/BP_CameraFollow.BP_CameraFollow_C"))
        (Game|Player|SetViewTargetwithBlend _returnvalue_2 _returnvalue_3 0.0 "VTBlend_Linear" 0.0 false)))))

(fn ConstructionScript)