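; Spear enemy pawn that patrols along X or swings its spear, and lets the player's snowball snap onto the tip.
; Chained timelines drive patrol, rotation and spear extend/retract, using trigonometry to move the hitbox, which Tick pins when idle.
; A hit with Space held attaches the player and possesses this pawn; releasing Space detaches and repossesses the player.
; Move inputs are stubs, with rotation logic left disconnected.
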(event OnComponentHit(hit_cube_collision)
  (params (HitComponent :type Primitive%20Component%20Object%20Reference) (OtherActor :type Actor%20Object%20Reference) (OtherComp :type Primitive%20Component%20Object%20Reference) (NormalImpulse :type Vector :default "0, 0, 0") (Hit :type Hit%20Result%20Structure%20%28by%20ref%29))
  (bind (_bblockinghit _binitialoverlap _time _distance _location _impactpoint _normal _impactnormal) (Collision|BreakHitResult Hit))
  (bind _hit_cube_collision (Variables|Components|Gethit_cube_collision))
  (bind (_x _y _z) (Math|Vector|BreakVector _impactpoint))
  (bind _returnvalue (* _impactnormal "-100.000000,-100.000000,-100.000000"))
  (bind _returnvalue_2 (+ _impactpoint _returnvalue))
  (bind (_x_2 _y_2 _z_2) (Math|Vector|BreakVector _returnvalue_2))
  ;[1 1 1] The snowball hit the spear extremity
  (bind _asbp_player_paw (Utilities|Casting|CastToBP_PlayerPaw OtherActor))
  (if (Variables|/Game/BluePrints/Player/BP_PlayerPaw.BP_PlayerPaw_C|GetisSpaceHold _asbp_player_paw)
    (bind _output_get (Variables|Default|SetanotherVector (Math|Vector|MakeVector (- _x_2 _x) (- _y_2 _y) (- _z_2 _z))))
    (Collision|LineTraceByChannel _impactpoint _returnvalue_2 "TraceTypeQuery1" false 0 "ForDuration" true "(R=1.000000,G=0.000000,B=0.000000,A=1.000000)" "(R=0.000000,G=1.000000,B=0.000000,A=1.000000)" 1e+01)
    (Utilities|FlowControl|DoOnce false
      (:Completed
        (Variables|Default|SetrectificationAngle (.Pitch (Math|Vector|GetYawPitchfromVector _output_get)))
        (Variables|/Game/BluePrints/Player/BP_PlayerPaw.BP_PlayerPaw_C|SetanchoredComponent _asbp_player_paw _hit_cube_collision)
        (Variables|Default|SetisSnap true)
        (Variables|/Game/BluePrints/Player/BP_PlayerPaw.BP_PlayerPaw_C|SetisSnap _asbp_player_paw true)
        (Variables|Components|SetattachedComponent (Variables|/Game/BluePrints/Player/BP_PlayerPaw.BP_PlayerPaw_C|GetCapsule _asbp_player_paw))
        (Transformation|AttachComponentToComponent (Variables|/Game/BluePrints/Player/BP_PlayerPaw.BP_PlayerPaw_C|GetCapsule _asbp_player_paw) _hit_cube_collision "SomeSocket" "KeepWorld" "KeepWorld" "KeepWorld" true)
        (Physics|SetSimulatePhysics (Variables|Components|Gethit_cube_collision) false)
        (bind _asbp_player_controller (Utilities|Casting|CastToBP_PlayerController (Game|GetPlayerController 0)))
        (Pawn|Possess _asbp_player_controller self)
        (Development|PrintString (Utilities|String|ToString(Float) (.pitch (Transformation|GetWorldRotation (Variables|/Game/BluePrints/Player/BP_PlayerPaw.BP_PlayerPaw_C|GetCapsule _asbp_player_paw)))) true true "(R=1.000000,G=0.179992,B=0.000000,A=1.000000)" 1e+01)
        (bind _returnvalue_3 (Actor|GetActorOfClass "/Game/BluePrints/Player/BP_CameraFollow.BP_CameraFollow_C"))
        (Game|Player|SetViewTargetwithBlend _asbp_player_controller _returnvalue_3 0.0 "VTBlend_Linear" 0.0 false)))))

(event Custom|SpearUp
  (bind _hit_cube_collision (Variables|Components|Gethit_cube_collision))
  (bind _relativerotation (Variables|/Script/Engine.SceneComponent|GetRelativeRotation _hit_cube_collision))
  (bind _relativelocation (Variables|/Script/Engine.SceneComponent|GetRelativeLocation _hit_cube_collision))
  (bind _returnvalue (Math|Rotator|GetRotationXVector _relativerotation))
  ;[1 1 1] spear up
  (Variables|Default|SetpreviousHitboxCollisionZValue _relativelocation)
  (Variables|Default|SetpreviousSpear1ZValue (Variables|/Script/Engine.SceneComponent|GetRelativeLocation (Variables|Components|Getspear1)))
  (Variables|Default|SetpreviousBox2ZValue (Variables|/Script/Engine.SceneComponent|GetRelativeLocation (Variables|Components|GetBox2)))
  (Variables|Default|SetfixHitboxCollisionLocation _relativelocation)
  (Variables|Default|SetfixHitboxCollisionRotation _returnvalue)
  (Variables|Default|SetisSpearDown false)
  (Variables|Default|SetsignSpearUp 1.0)
  (Variables|Default|SetisHitboxCollisionMoving false)
  (Variables|Default|SetisHitboxCollisionMoving true)
  (bind _spearuptrack (Timeline|SpearUpTimeline PlayFromStart)
    (:Update
      (Transformation|SetRelativeLocation (Variables|Components|Getspear1) (Math|Vector|MakeVector 0.0 (+ (.y (Variables|Default|GetpreviousSpear1ZValue)) (* (* (Math|Trig|Sin(Degrees) (Variables|Default|GetrelRotY)) (Variables|Default|GetspearUpPower) (Variables|Default|GetsignSpearUp) _spearuptrack) -1.0)) (+ (.z (Variables|Default|GetpreviousSpear1ZValue)) (* (* (Math|Trig|Cos(Degrees) (Variables|Default|GetrelRotY)) (Variables|Default|GetspearUpPower) (Variables|Default|GetsignSpearUp) _spearuptrack) -1.0))) false false)
      (Transformation|SetRelativeLocation (Variables|Components|GetBox2) (Math|Vector|MakeVector (+ (.x (Variables|Default|GetpreviousBox2ZValue)) (* (* (* (Math|Trig|Sin(Degrees) (Variables|Default|GetrelRotY)) (Variables|Default|GetspearUpPower) (Variables|Default|GetsignSpearUp) _spearuptrack) -1.0) 1.0) (* (.z (Variables|Default|GetpreviousBox2ZValue)) -1.0)) 0.0 (.z (Variables|Default|GetpreviousBox2ZValue))) false false)
      (Transformation|SetRelativeLocation (Variables|Components|Gethit_cube_collision) (Math|Vector|MakeVector (+ (* (* (* (Math|Trig|Sin(Degrees) (Variables|Default|GetrelRotY)) (Variables|Default|GetspearUpPower) (Variables|Default|GetsignSpearUp) _spearuptrack) -1.0) 1.0) (.x (Variables|Default|GetpreviousHitboxCollisionZValue)) 0.0) 0.0 (.z (Variables|Default|GetpreviousHitboxCollisionZValue))) false false))
    (:Finished
      (Variables|Default|SetfixHitboxCollisionLocation _relativelocation)
      (Variables|Default|SetfixHitboxCollisionRotation _returnvalue)
      (Variables|Default|SetisHitboxCollisionMoving false)
      (if (Variables|Default|GetisSpearDown)
        (if (Variables|Default|GetisEnemySpearUp)
          (Utilities|FlowControl|FlipFlop
            (:A
              (CallFunction|RotateSpearOFF))
            (:B
              (CallFunction|RotateSpearON)))
          (else
            (CallFunction|RotateSpearOFF)))
        (else
          (Utilities|FlowControl|Delay (Variables|Default|GettimeBetweenSpearSwitch))
          (Variables|Default|SetisHitboxCollisionMoving true)
          (Variables|Default|SetsignSpearUp -1.0)
          (Variables|Default|SetisSpearDown true)
          (Variables|Default|SetpreviousSpear1ZValue (Math|Vector|MakeVector 0.0 (+ (.y (Variables|Default|GetpreviousSpear1ZValue)) (* (Math|Trig|Sin(Degrees) (Variables|Default|GetrelRotY)) (Variables|Default|GetspearUpPower) (Variables|Default|GetsignSpearUp) 1.0)) (+ (.z (Variables|Default|GetpreviousSpear1ZValue)) (* (Math|Trig|Cos(Degrees) (Variables|Default|GetrelRotY)) (Variables|Default|GetspearUpPower) (Variables|Default|GetsignSpearUp) 1.0))))
          (Variables|Default|SetpreviousHitboxCollisionZValue (Math|Vector|MakeVector (+ (.x (Variables|Default|GetpreviousHitboxCollisionZValue)) (* (Math|Trig|Sin(Degrees) (Variables|Default|GetrelRotY)) (Variables|Default|GetspearUpPower) (Variables|Default|GetsignSpearUp) 1.0)) 0.0 (.z (Variables|Default|GetpreviousHitboxCollisionZValue))))
          (Variables|Default|SetpreviousBox2ZValue (Math|Vector|MakeVector (+ (+ (* (Math|Trig|Sin(Degrees) (Variables|Default|GetrelRotY)) (Variables|Default|GetspearUpPower) (Variables|Default|GetsignSpearUp) 1.0) (.x (Variables|Default|GetpreviousBox2ZValue))) (* (.z (Variables|Default|GetpreviousBox2ZValue)) -1.0)) 0.0 (.z (Variables|Default|GetpreviousBox2ZValue))))
          (Timeline|SpearUpTimeline PlayFromStart))))))

(event Custom|RotateSpearON
  (bind _box2 (Variables|Components|GetBox2))
  (bind _hit_cube_collision (Variables|Components|Gethit_cube_collision))
  (bind _hit_cube_collision_2 (Variables|Components|Gethit_cube_collision))
  (bind _returnvalue (Transformation|GetWorldLocation _box2))
  ;[1 1 1] rotate
  (Utilities|FlowControl|Delay (Variables|Default|GettimeBetweenSpearRotate))
  (Variables|Default|SetisHitboxCollisionMoving true)
  (Variables|Default|SetisRotateSpear true)
  (if (> (Variables|Default|GetrotationDirection) 0.0)
    (bind _newtrack_0 (Timeline|Timeline_1 PlayFromStart)
      (:Update
        (Transformation|SetRelativeRotation (Variables|Components|Get%20Head) (Math|Rotator|MakeRotator (.roll (Variables|/Script/Engine.SceneComponent|GetRelativeRotation (Variables|Components|Get%20Head))) (* _newtrack_0 (Variables|Default|GetrelRotY)) 0.0) false false)
        (Transformation|SetRelativeLocation _box2 (Math|Vector|MakeVector (* (Math|Trig|Cos(Degrees) (+ (* _newtrack_0 (Variables|Default|GetrelRotY)) 9e+01)) 94.0) 0.0 (* (Math|Trig|Sin(Degrees) (+ (* _newtrack_0 (Variables|Default|GetrelRotY)) 9e+01)) 94.0)) false false)
        (Transformation|SetRelativeRotation _box2 (Math|Rotator|MakeRotator 0.0 (* _newtrack_0 (Variables|Default|GetrelRotY)) 0.0) false false)
        (Transformation|SetWorldLocation _hit_cube_collision (Math|Vector|MakeVector (+ (.x _returnvalue) (* (Math|Trig|Cos(Degrees) (+ (* _newtrack_0 (Variables|Default|GetrelRotY)) 9e+01)) 2.0)) 0.0 (+ (.z _returnvalue) (* (Math|Trig|Sin(Degrees) (+ (* _newtrack_0 (Variables|Default|GetrelRotY)) 9e+01)) 2.0))) false false)
        (Transformation|SetWorldRotation _hit_cube_collision (Math|Rotator|MakeRotator 0.0 (* _newtrack_0 (Variables|Default|GetrelRotY)) 0.0) false false))
      (:Finished
        (Variables|Default|SetfixHitboxCollisionLocation (Variables|/Script/Engine.SceneComponent|GetRelativeLocation _hit_cube_collision_2))
        (Variables|Default|SetfixHitboxCollisionRotation (Math|Rotator|GetRotationXVector (Variables|/Script/Engine.SceneComponent|GetRelativeRotation _hit_cube_collision_2)))
        (Variables|Default|SetisHitboxCollisionMoving false)
        (if (Variables|Default|GetisRotateSpear)
          (CallFunction|SpearUp)
          (elif (Variables|Default|GetisEnemySpearUp)
            (CallFunction|SpearUp)
            (else
              (CallFunction|RotateSpearON))))))))

(event Custom|rotateSpearOFF
  (bind _box2 (Variables|Components|GetBox2))
  (bind _hit_cube_collision (Variables|Components|Gethit_cube_collision))
  (bind _hit_cube_collision_2 (Variables|Components|Gethit_cube_collision))
  (bind _returnvalue (Transformation|GetWorldLocation _box2))
  ;[1 1 1] rotate
  (Utilities|FlowControl|Delay (Variables|Default|GettimeBetweenSpearRotate))
  (Variables|Default|SetisHitboxCollisionMoving true)
  (if (Variables|Default|GetisRotateSpear)
    (Variables|Default|SetisRotateSpear false)
    (bind _newtrack_0 (Timeline|Timeline_1 ReverseFromEnd)
      (:Update
        (Transformation|SetRelativeRotation (Variables|Components|Get%20Head) (Math|Rotator|MakeRotator (.roll (Variables|/Script/Engine.SceneComponent|GetRelativeRotation (Variables|Components|Get%20Head))) (* _newtrack_0 (Variables|Default|GetrelRotY)) 0.0) false false)
        (Transformation|SetRelativeLocation _box2 (Math|Vector|MakeVector (* (Math|Trig|Cos(Degrees) (+ (* _newtrack_0 (Variables|Default|GetrelRotY)) 9e+01)) 94.0) 0.0 (* (Math|Trig|Sin(Degrees) (+ (* _newtrack_0 (Variables|Default|GetrelRotY)) 9e+01)) 94.0)) false false)
        (Transformation|SetRelativeRotation _box2 (Math|Rotator|MakeRotator 0.0 (* _newtrack_0 (Variables|Default|GetrelRotY)) 0.0) false false)
        (Transformation|SetWorldLocation _hit_cube_collision (Math|Vector|MakeVector (+ (.x _returnvalue) (* (Math|Trig|Cos(Degrees) (+ (* _newtrack_0 (Variables|Default|GetrelRotY)) 9e+01)) 2.0)) 0.0 (+ (.z _returnvalue) (* (Math|Trig|Sin(Degrees) (+ (* _newtrack_0 (Variables|Default|GetrelRotY)) 9e+01)) 2.0))) false false)
        (Transformation|SetWorldRotation _hit_cube_collision (Math|Rotator|MakeRotator 0.0 (* _newtrack_0 (Variables|Default|GetrelRotY)) 0.0) false false))
      (:Finished
        (Variables|Default|SetfixHitboxCollisionLocation (Variables|/Script/Engine.SceneComponent|GetRelativeLocation _hit_cube_collision_2))
        (Variables|Default|SetfixHitboxCollisionRotation (Math|Rotator|GetRotationXVector (Variables|/Script/Engine.SceneComponent|GetRelativeRotation _hit_cube_collision_2)))
        (Variables|Default|SetisHitboxCollisionMoving false)
        (if (Variables|Default|GetisRotateSpear)
          (CallFunction|SpearUp)
          (elif (Variables|Default|GetisEnemySpearUp)
            (CallFunction|SpearUp)
            (else
              (CallFunction|RotateSpearON))))))))

(event Input|EnhancedActionEvents|EnhancedInputActionBP_Free
  (params (ActionValue :type Boolean) (ElapsedSeconds :type Float%20%28double-precision%29) (TriggeredSeconds :type Float%20%28double-precision%29) (InputAction :type Input%20Action%20Object%20Reference :default "/Game/BluePrints/Player/inputs/BP_Free.BP_Free")))

(event Input|EnhancedActionEvents|EnhancedInputActionBP_Move
  (params (ActionValue :type Vector :default "0, 0, 0") (ElapsedSeconds :type Float%20%28double-precision%29) (TriggeredSeconds :type Float%20%28double-precision%29) (InputAction :type Input%20Action%20Object%20Reference :default "/Game/BluePrints/Player/inputs/BP_Move.BP_Move"))
  ;[1 1 1] rotate hit cube attached between two angles
  (:Triggered
    (if (Variables|Default|GetisSnap) :!label _label
      _))
  (:Started
    (goto _label))
  (:Ongoing
    (goto _label)))

(event Input|EnhancedActionEvents|EnhancedInputActionBP_RightMove
  (params (ActionValue :type Vector :default "0, 0, 0") (ElapsedSeconds :type Float%20%28double-precision%29) (TriggeredSeconds :type Float%20%28double-precision%29) (InputAction :type Input%20Action%20Object%20Reference :default "/Game/BluePrints/Player/inputs/BP_RightMove.BP_RightMove"))
  ;[1 1 1] rotate hit cube attached between two angles
  (:Triggered
    (if (Variables|Default|GetisSnap) :!label _label
      _))
  (:Started
    (goto _label))
  (:Ongoing
    (goto _label)))

(event EventBeginPlay
  (bind _defaultsceneroot (Variables|Components|GetDefaultSceneRoot))
  (bind _hit_cube_collision (Variables|Components|Gethit_cube_collision))
  (bind _box2 (Variables|Components|GetBox2))
  (bind _returnvalue (Transformation|GetWorldLocation _box2))
  (bind _returnvalue_2 (Transformation|GetWorldLocation _hit_cube_collision))
  (bind _returnvalue_3 (Transformation|GetWorldLocation _defaultsceneroot))
  ;[1 1 1] Move component between two points described by distance between them
  (Variables|Default|SetprevRelRotY (Variables|Default|GetrelRotY))
  (if (== (Variables|Default|GetrotationDirection) 0.0)
    (Variables|Default|SetstartLocationX (.x _returnvalue_3) :!label _label)
    (Variables|Default|SetrelLocHitCube (Variables|/Script/Engine.SceneComponent|GetRelativeLocation (Variables|Components|GetBox2)))
    (Utilities|FlowControl|Delay (Variables|Default|GetdelayBetweenPatrol))
    (Components|Timeline|SetPlayRate (Variables|Default|GetTimeline) (Variables|Default|GetpatrolRate))
    (bind _newtrack_0 (Timeline|Timeline PlayFromStart)
      (:Update
        (Transformation|SetWorldLocation (Variables|Components|GetDefaultSceneRoot) (Math|Vector|MakeVector (+ (Variables|Default|GetstartLocationX) (* _newtrack_0 (Variables|Default|GetenemyDistancePatrol))) 0.0 (.z _returnvalue_3)) false false)
        (Transformation|SetWorldLocation (Variables|Components|GetBox2) (Math|Vector|MakeVector (+ (Variables|Default|GetstartLocationX) (* _newtrack_0 (Variables|Default|GetenemyDistancePatrol))) 0.0 (.z _returnvalue)) false false)
        (Transformation|SetWorldLocation _hit_cube_collision (Math|Vector|MakeVector (+ (Variables|Default|GetstartLocationX) (* _newtrack_0 (Variables|Default|GetenemyDistancePatrol))) 0.0 (.z _returnvalue_2)) false false))
      (:Finished
        (if (Variables|Default|GetisEnemySpearUp)
          (CallFunction|SpearUp))
        (bind _output_get (Variables|Default|SetstartLocationX (.x _returnvalue_3)))
        (Utilities|FlowControl|Delay (Variables|Default|GetdelayBetweenPatrol))
        (Components|Timeline|SetPlayRate (Variables|Default|GetTimeline_0) (Variables|Default|GetpatrolRate))
        (bind _newtrack_0_2 (Timeline|Timeline_0 PlayFromStart)
          (:Update
            (Transformation|SetWorldLocation (Variables|Components|GetDefaultSceneRoot) (Math|Vector|MakeVector (- _output_get (* _newtrack_0_2 (Variables|Default|GetenemyDistancePatrol))) 0.0 (.z _returnvalue_3)) false false)
            (Transformation|SetWorldLocation (Variables|Components|GetBox2) (Math|Vector|MakeVector (- _output_get (* _newtrack_0_2 (Variables|Default|GetenemyDistancePatrol))) 0.0 (.z _returnvalue)) false false)
            (Transformation|SetWorldLocation (Variables|Components|Gethit_cube_collision) (Math|Vector|MakeVector (- _output_get (* _newtrack_0_2 (Variables|Default|GetenemyDistancePatrol))) 0.0 (.z _returnvalue_2)) false false))
          (:Finished
            (if (Variables|Default|GetisEnemySpearUp)
              (CallFunction|SpearUp)
              (goto _label)
              (else
                (goto _label)))))))
    (else
      (Utilities|FlowControl|Delay (Variables|Default|GettimeBetweenSpearRotate))
      (CallFunction|RotateSpearON))))

(event EventTick
  (params (DeltaSeconds :type Float%20%28single-precision%29))
  (bind _hit_cube_collision (Variables|Components|Gethit_cube_collision))
  (if (not (Variables|Default|GetisHitboxCollisionMoving))
    (if (or (Utilities|Operators|NotEqual(!=) (Variables|/Script/Engine.SceneComponent|GetRelativeRotation _hit_cube_collision) (Variables|Default|GetfixHitboxCollisionRotation) 0.0) (Class|KismetMathLibrary|NotEqualExactlyVectorVector (Variables|/Script/Engine.SceneComponent|GetRelativeLocation _hit_cube_collision) (Variables|Default|GetfixHitboxCollisionLocation)))
      (Transformation|SetRelativeLocation _hit_cube_collision (Variables|Default|GetfixHitboxCollisionLocation) false false)
      (Transformation|SetRelativeRotation _hit_cube_collision (Math|Conversions|RotationFromXVector (Variables|Default|GetfixHitboxCollisionRotation)) false false))))

(event Input|KeyboardEvents|SpaceBar
  (params (Key :type Key%20Structure))
  (bind _hit_cube_collision (Variables|Components|Gethit_cube_collision))
  ;[1 1 1] Forcément là puisque c'est ici que les contrôles ont lieu!
  (:Released
    (Utilities|FlowControl|DoOnce false :!label _label
      (:Completed
        (bind _returnvalue (Actor|GetActorOfClass "/Game/BluePrints/Player/BP_PlayerPaw.BP_PlayerPaw_C"))
        (Default|ResetSpaceHold _returnvalue)
        (Development|PrintString "space bar pressed")
        (Transformation|DetachFromComponent (Variables|/Game/BluePrints/Player/BP_PlayerPaw.BP_PlayerPaw_C|GetCapsule _returnvalue) "KeepWorld" "KeepWorld" "KeepWorld" true)
        (Physics|SetSimulatePhysics (Variables|Components|Gethit_cube_collision) false)
        (bind _returnvalue_2 (Actor|GetActorOfClass "/Game/BluePrints/Player/BP_PlayerController.BP_PlayerController_C"))
        (Pawn|Possess _returnvalue_2 _returnvalue)
        (Physics|SetSimulatePhysics (Variables|/Game/BluePrints/Player/BP_PlayerPaw.BP_PlayerPaw_C|GetCapsule _returnvalue) true)
        (bind _returnvalue_3 (Actor|GetActorOfClass "/Game/BluePrints/Player/BP_CameraFollow.BP_CameraFollow_C"))
        (Game|Player|SetViewTargetwithBlend _returnvalue_2 _returnvalue_3 0.0 "VTBlend_Linear" 0.0 false)
        (Utilities|FlowControl|Delay 2.0)
        (Utilities|FlowControl|Sequence
          (:then_0
            ;[1 1 1] The snowball hit the spear extremity
            (Utilities|FlowControl|DoOnce false) ; enters at Reset
          )
          (:then_1
            (goto _label Reset)))))))

(fn ConstructionScript)