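; A switch-triggered door that opens once when CallSwitchDoor fires, swapping its Cube material and playing a timeline at MovingRate.
; Coor picks the axis: X lerps the Box between spline endpoints, while Z lerps from its current height toward a rise equal to the spline's length.
; On finish, it stops a BP_SimpleSnowMovingPlatform whose AttributedSwitch matches AttributedSwitchName.
; CloseGate only prints a debug string.
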(event Custom|CallSwitchDoor
  (bind _box (Variables|Default|GetBox))
  (bind _coor (Variables|Default|Getcoor))
  (bind _movementspline (Variables|Default|GetMovementSpline))
  (bind _returnvalue (Transformation|GetWorldLocation _box))
  (Utilities|FlowControl|DoOnce false
    (:Completed
      (Variables|Default|SetisOpen true)
      (Rendering|Material|SetMaterial (Variables|Default|GetCube) 0 "/Engine/MapTemplates/Materials/BasicAsset03.BasicAsset03")
      (Components|Timeline|SetPlayRate (Variables|Default|GetTimeline) (Variables|Default|GetmovingRate))
      (Variables|Default|SetnewZ (+ (.z _returnvalue) (Spline|GetSplineLength _movementspline)))
      (bind _alpha (Timeline|Timeline PlayFromStart)
        (:Update
          (if (Utilities|Enum|Equal(Enum) _coor "x")
            (Transformation|SetWorldLocation _box (Math|Vector|MakeVector (Math|Float|Lerp (.x (Class|SplineComponent|GetLocationatSplineInputKey _movementspline 0.0 "World")) (.x (Class|SplineComponent|GetLocationatSplineInputKey _movementspline 1.0 "World")) _alpha) 0.0 (.z (Transformation|GetWorldLocation _box))) false false)
            (elif (Utilities|Enum|Equal(Enum) _coor "z")
              (Transformation|SetWorldLocation _box (Math|Vector|MakeVector (.x _returnvalue) 0.0 (Math|Float|Lerp (.z _returnvalue) (Variables|Default|GetnewZ) _alpha)) false false))))
        (:Finished
          (bind _outactors (Actor|GetAllActorsOfClass "/Game/BluePrints/Platforms/BP_SimpleSnowMovingPlatform.BP_SimpleSnowMovingPlatform_C"))
          (bind _array_element (Utilities|Array|ForEachLoopwithBreak _outactors :!label _label)
            (:LoopBody
              (if (Utilities|Enum|Equal(Enum) (Variables|/Game/BluePrints/Platforms/BP_SimpleSnowMovingPlatform.BP_SimpleSnowMovingPlatform_C|GetAttributedSwitch _array_element) (Variables|Default|GetAttributedSwitchName))
                (Utilities|FlowControl|DoOnce false
                  (:Completed
                    (Variables|/Game/BluePrints/Platforms/BP_SimpleSnowMovingPlatform.BP_SimpleSnowMovingPlatform_C|SetisStop _array_element true)
                    (Audio|Components|Audio|Stop (Variables|/Game/BluePrints/Platforms/BP_SimpleSnowMovingPlatform.BP_SimpleSnowMovingPlatform_C|GetTimeline _array_element))
                    (goto _label Break)))))))))))

(event Custom|CloseGate
  (Development|PrintString "CloseGate"))

(event EventBeginPlay)

(event Collision|EventActorBeginOverlap
  (params (OtherActor :type Actor%20Object%20Reference)))

(event EventTick
  (params (DeltaSeconds :type Float%20%28single-precision%29)))

(fn ConstructionScript)