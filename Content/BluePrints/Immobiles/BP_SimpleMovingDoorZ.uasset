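; Vertical moving door that doubles as an elevator, triggered by overlapping its Box.
; Overlap changes the Cube's material and plays a Timeline that lerps the Box's Z between MovementSpline's first two points.
; In elevator mode, leaving the Box re-arms the trigger and reverses the Timeline if travel is near either end.
; DoOnce gates and IsElevatorReversed block retriggers, with the flag clearing after a return from the top and a short delay.
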(event OnComponentBeginOverlap(Box)
  (params (OverlappedComponent :type Primitive%20Component%20Object%20Reference) (OtherActor :type Actor%20Object%20Reference) (OtherComp :type Primitive%20Component%20Object%20Reference) (OtherBodyIndex :type Integer) (bFromSweep :type Boolean) (SweepResult :type Hit%20Result%20Structure%20%28by%20ref%29))
  (bind _box (Variables|Default|GetBox))
  (bind _movementspline (Variables|Default|GetMovementSpline))
  (bind _returnvalue (Class|SplineComponent|GetLocationatSplineInputKey _movementspline 1.0 "Local"))
  (if (not (Variables|Default|GetisElevatorReversed))
    (Utilities|FlowControl|DoOnce false
      (:Completed
        (Utilities|FlowControl|Sequence
          (:then_0
            (Utilities|FlowControl|DoOnce false) ; enters at Reset
          )
          (:then_1
            (Rendering|Material|SetMaterial (Variables|Default|GetCube) 0 "/Engine/MapTemplates/Materials/BasicAsset03.BasicAsset03")
            (Components|Timeline|SetPlayRate (Variables|Default|GetTimeline) (Variables|Default|GetmovingRate))
            (bind _alpha (Timeline|Timeline PlayFromStart)
              (:Update
                (Variables|Default|SetdistanceParcourue (Math|Float|Lerp (.z (Class|SplineComponent|GetLocationatSplineInputKey _movementspline 0.0 "Local")) (.z _returnvalue) _alpha))
                (Transformation|SetRelativeLocation _box (Math|Vector|MakeVector (.x (Variables|/Script/Engine.SceneComponent|GetRelativeLocation _box)) 0.0 (Math|Float|Lerp (.z (Class|SplineComponent|GetLocationatSplineInputKey _movementspline 0.0 "Local")) (.z _returnvalue) _alpha)) false false))
              (:Finished
                (if (Variables|Default|GetisElevatorReversed)
                  (Utilities|FlowControl|Delay 1.0)
                  (Development|PrintString "Elevator has been reset successfully")
                  (Variables|Default|SetisElevatorReversed false))))))))))

(event OnComponentEndOverlap(Box)
  (params (OverlappedComponent :type Primitive%20Component%20Object%20Reference) (OtherActor :type Actor%20Object%20Reference) (OtherComp :type Primitive%20Component%20Object%20Reference) (OtherBodyIndex :type Integer))
  (bind _box (Variables|Default|GetBox))
  (bind _movementspline (Variables|Default|GetMovementSpline))
  (bind _returnvalue (Class|SplineComponent|GetLocationatSplineInputKey _movementspline 1.0 "Local"))
  (if (Variables|Default|GetisElevator)
    (if true
      (Utilities|FlowControl|DoOnce false
        (:Completed
          (Utilities|FlowControl|Sequence
            (:then_0
              (Utilities|FlowControl|DoOnce false) ; enters at Reset
            )
            (:then_1
              (if (<= (Math|Float|Absolute(Float) (Variables|Default|GetdistanceParcourue)) 5.0)
                (bind _alpha (Timeline|Timeline Reverse)
                  (:Update
                    (Variables|Default|SetdistanceParcourue (Math|Float|Lerp (.z (Class|SplineComponent|GetLocationatSplineInputKey _movementspline 0.0 "Local")) (.z _returnvalue) _alpha))
                    (Transformation|SetRelativeLocation _box (Math|Vector|MakeVector (.x (Variables|/Script/Engine.SceneComponent|GetRelativeLocation _box)) 0.0 (Math|Float|Lerp (.z (Class|SplineComponent|GetLocationatSplineInputKey _movementspline 0.0 "Local")) (.z _returnvalue) _alpha)) false false))
                  (:Finished
                    (if (Variables|Default|GetisElevatorReversed)
                      (Utilities|FlowControl|Delay 1.0)
                      (Development|PrintString "Elevator has been reset successfully")
                      (Variables|Default|SetisElevatorReversed false))))
                (elif (>= (Math|Float|Absolute(Float) (Variables|Default|GetdistanceParcourue)) (- (.z _returnvalue) 5.0))
                  (Variables|Default|SetisElevatorReversed true)
                  (Timeline|Timeline ReverseFromEnd))))))))))

(event EventBeginPlay)

(event Collision|EventActorBeginOverlap
  (params (OtherActor :type Actor%20Object%20Reference)))

(event EventTick
  (params (DeltaSeconds :type Float%20%28single-precision%29)))

(fn ConstructionScript)