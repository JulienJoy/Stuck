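; BP_Spike is a spike hazard that reloads the saved game through GM_Stuck when the player pawn overlaps its capsule.
; On BeginPlay, spikes flagged IsSaint swap to the saint sprite and clear the second sprite.
; Setting IsLookingToPlayer makes Tick orient the cone from a look-at rotation once, then reset the flag.
; MoveFromTheGroundThenDestroy raises the spike on a timeline, using a FlipFlop to retract it faster before destroying it.
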(event OnComponentBeginOverlap(Capsule)
  (params (OverlappedComponent :type Primitive%20Component%20Object%20Reference) (OtherActor :type Actor%20Object%20Reference) (OtherComp :type Primitive%20Component%20Object%20Reference) (OtherBodyIndex :type Integer) (bFromSweep :type Boolean) (SweepResult :type Hit%20Result%20Structure%20%28by%20ref%29))
  (Utilities|Casting|CastToBP_PlayerPaw OtherActor)
  ;[1 0.4074 0] ICI
  (bind _asgm_stuck (Utilities|Casting|CastToGM_Stuck (Game|GetGameMode)))
  (Default|LoadGame _asgm_stuck))

(event Custom|MoveFromTheGroundThenDestroy
  (bind _returnvalue (Transformation|GetActorLocation))
  (Utilities|FlowControl|Delay 0.2)
  (Variables|Default|SetpreviousSpikeZ (.z _returnvalue))
  (Components|Timeline|SetPlayRate (Variables|Default|GetTimeline) 3.0)
  (bind _z (Timeline|Timeline PlayFromStart)
    (:Update
      (Transformation|SetActorLocation (Math|Vector|MakeVector (.x _returnvalue) (.y _returnvalue) (Math|Float|Lerp (Variables|Default|GetpreviousSpikeZ) (+ (Variables|Default|GetpreviousSpikeZ) 1.1e+02) _z)) false false))
    (:Finished
      (Utilities|FlowControl|FlipFlop
        (:A
          (Components|Timeline|SetPlayRate (Variables|Default|GetTimeline) 2e+01)
          (Timeline|Timeline ReverseFromEnd))
        (:B
          (Actor|DestroyActor))))))

(event Custom|ChangeMaterialToSaint
  (Rendering|Components|Sprite|SetSprite (Variables|Default|GetPaperSprite) "/Game/BluePrints/Immobiles/picsaint_Sprite.picsaint_Sprite")
  (Rendering|Components|Sprite|SetSprite (Variables|Default|GetPaperSprite1) 0))

(event Custom|ConditionCheckChangeMaterialToSaint
  (if (Variables|Default|GetisSaint)
    (CallFunction|ChangeMaterialtoSaint)))

(event EventBeginPlay
  (CallFunction|ConditionCheckChangeMaterialtoSaint))

(event Collision|EventActorBeginOverlap
  (params (OtherActor :type Actor%20Object%20Reference)))

(event EventTick
  (params (DeltaSeconds :type Float%20%28single-precision%29))
  (bind _returnvalue (Game|Player|GetPlayerPawn 0))
  (bind _cone (Variables|Default|GetCone))
  (bind _rectificationrotator (Variables|Default|GetrectificationRotator))
  (bind _returnvalue_2 (Transformation|GetActorLocation _returnvalue))
  (bind _returnvalue_3 (Transformation|GetWorldLocation _cone))
  (bind _returnvalue_4 (Math|Rotator|FindLookatRotation _returnvalue_3 _returnvalue_2))
  (bind _returnvalue_5 (+ (.roll _returnvalue_4) 1.8e+02))
  (bind _returnvalue_6 (+ _returnvalue_5 _rectificationrotator))
  (if (Variables|Default|GetisLookingToPlayer)
    (Transformation|SetWorldRotation _cone (Math|Rotator|MakeRotator _returnvalue_6 (+ (.pitch _returnvalue_4) _rectificationrotator) _returnvalue_6) false false)
    (Variables|Default|SetisLookingToPlayer false)))

(fn ConstructionScript)