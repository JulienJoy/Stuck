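; BP_SwitchSimpleMovingDoor is a one-shot switch that activates moving doors or a platform when BP_PlayerPaw hits its Cube.
; The first hit swaps the sprite and material to the ON look.
; A hardcoded SwitchName "switch2" calls the first BP_SimpleSnowMovingPlatform with a matching AttributedSwitch.
; Any other name calls every BP_SimpleMovingDoor with a matching AttributedSwitchName, both found through GetAllActorsOfClass.
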(event OnComponentHit(Cube)
  (params (HitComponent :type Primitive%20Component%20Object%20Reference) (OtherActor :type Actor%20Object%20Reference) (OtherComp :type Primitive%20Component%20Object%20Reference) (NormalImpulse :type Vector :default "0, 0, 0") (Hit :type Hit%20Result%20Structure%20%28by%20ref%29))
  (Utilities|Casting|CastToBP_PlayerPaw OtherActor)
  (Utilities|FlowControl|DoOnce false
    (:Completed
      (Rendering|Components|Sprite|SetSprite (Variables|Default|GetPaperSprite) "/Game/BluePrints/Immobiles/switchSimpleDoorBlueON_Sprite.switchSimpleDoorBlueON_Sprite")
      (Rendering|Material|SetMaterial (Variables|Default|GetCube) 0 "/Engine/MapTemplates/Materials/BasicAsset03.BasicAsset03")
      (if (Utilities|Enum|Equal(Enum) (Variables|Default|GetswitchName) "switch2")
        (bind _outactors (Actor|GetAllActorsOfClass "/Game/BluePrints/Platforms/BP_SimpleSnowMovingPlatform.BP_SimpleSnowMovingPlatform_C"))
        (bind _array_element (Utilities|Array|ForEachLoopwithBreak _outactors :!label _label)
          (:LoopBody
            (if (Utilities|Enum|Equal(Enum) (Variables|/Game/BluePrints/Platforms/BP_SimpleSnowMovingPlatform.BP_SimpleSnowMovingPlatform_C|GetAttributedSwitch _array_element) (Variables|Default|GetswitchName))
              (Default|CallSwitchPlatform _array_element)
              (goto _label Break))))
        (else
          (bind _outactors_2 (Actor|GetAllActorsOfClass "/Game/BluePrints/Immobiles/BP_SimpleMovingDoor.BP_SimpleMovingDoor_C"))
          (for _array_element_2 _outactors_2
            (if (Utilities|Enum|Equal(Enum) (Variables|/Game/BluePrints/Immobiles/BP_SimpleMovingDoor.BP_SimpleMovingDoor_C|GetAttributedSwitchName _array_element_2) (Variables|Default|GetswitchName))
              (Default|CallSwitchDoor _array_element_2))))))))

(event EventBeginPlay)

(event Collision|EventActorBeginOverlap
  (params (OtherActor :type Actor%20Object%20Reference)))

(event EventTick
  (params (DeltaSeconds :type Float%20%28single-precision%29)))

(fn ConstructionScript)