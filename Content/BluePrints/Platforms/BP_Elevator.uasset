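; BP_Elevator is a platform that rises or descends while the player pawn (BP_PlayerPaw) is inside its trigger Box.
; Begin overlap plays ElevatorTimeline after a two-second delay, and end overlap reverses it after the same delay.
; The timeline track scales FalseCube1's relative location to drive only Cube's Z, so FalseCube1 marks the travel height.
; ElevatorSpeed sets the timeline play rate at BeginPlay.
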(event OnComponentBeginOverlap(Box)
  (params (OverlappedComponent :type Primitive%20Component%20Object%20Reference) (OtherActor :type Actor%20Object%20Reference) (OtherComp :type Primitive%20Component%20Object%20Reference) (OtherBodyIndex :type Integer) (bFromSweep :type Boolean) (SweepResult :type Hit%20Result%20Structure%20%28by%20ref%29))
  (bind _cube (Variables|Default|GetCube))
  (bind _relativelocation (Variables|/Script/Engine.SceneComponent|GetRelativeLocation _cube))
  (Utilities|Casting|CastToBP_PlayerPaw OtherActor)
  (Utilities|FlowControl|Delay 2.0)
  (bind _newtrack_1 (Timeline|ElevatorTimeline Play)
    (:Update
      (Transformation|SetRelativeLocation _cube (Math|Vector|MakeVector (.x _relativelocation) (.y _relativelocation) (.z (* _newtrack_1 (Variables|/Script/Engine.SceneComponent|GetRelativeLocation (Variables|Default|GetFalseCube1))))) false false))))

(event OnComponentEndOverlap(Box)
  (params (OverlappedComponent :type Primitive%20Component%20Object%20Reference) (OtherActor :type Actor%20Object%20Reference) (OtherComp :type Primitive%20Component%20Object%20Reference) (OtherBodyIndex :type Integer))
  (bind _cube (Variables|Default|GetCube))
  (bind _relativelocation (Variables|/Script/Engine.SceneComponent|GetRelativeLocation _cube))
  (Utilities|Casting|CastToBP_PlayerPaw OtherActor)
  (Utilities|FlowControl|Delay 2.0)
  (bind _newtrack_1 (Timeline|ElevatorTimeline Reverse)
    (:Update
      (Transformation|SetRelativeLocation _cube (Math|Vector|MakeVector (.x _relativelocation) (.y _relativelocation) (.z (* _newtrack_1 (Variables|/Script/Engine.SceneComponent|GetRelativeLocation (Variables|Default|GetFalseCube1))))) false false))))

(event EventBeginPlay
  (Components|Timeline|SetPlayRate (Variables|Default|GetElevatorTimeline) (Variables|Default|GetelevatorSpeed)))

(fn ConstructionScript)