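; BP_SimpleMovingPlatform is a platform that shuttles back and forth along a spline, starting on BeginPlay.
; A Timeline alpha interpolates distance along MovementSpline, and each update sets the Box component's world location to that point without sweeping.
; The Timeline's Finished output feeds back into a FlipFlop that alternates play from start and reverse from end, giving an endless ping-pong loop.
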(event EventBeginPlay
  (bind _movementspline (Variables|Default|GetMovementSpline))
  (Utilities|FlowControl|FlipFlop :!label _label
    (:A
      (bind _alpha (Timeline|Timeline PlayFromStart)
        (:Update
          (Transformation|SetWorldLocation (Variables|Default|GetBox) (Spline|GetLocationatDistanceAlongSpline _movementspline (Math|Float|Lerp 0.0 (Spline|GetSplineLength _movementspline) _alpha) "World") false false))
        (:Finished
          (goto _label))))
    (:B
      (Timeline|Timeline ReverseFromEnd))))

(event Collision|EventActorBeginOverlap
  (params (OtherActor :type Actor%20Object%20Reference)))

(event EventTick
  (params (DeltaSeconds :type Float%20%28single-precision%29)))

(fn ConstructionScript)