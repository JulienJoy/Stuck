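; Snow-themed moving platform that carries its Cube along a spline via a timeline.
; It moves on BeginPlay at a set rate or, if not set to, starts on the player paw's first hit.
; CallSwitchPlatform removes the optional right wall, sets the stop flag and replays the movement.
; The paw's first overlap with the Snowpile zeroes its capsule's physics velocity.
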(event OnComponentHit(Cube)
  (params (HitComponent :type Primitive%20Component%20Object%20Reference) (OtherActor :type Actor%20Object%20Reference) (OtherComp :type Primitive%20Component%20Object%20Reference) (NormalImpulse :type Vector :default "0, 0, 0") (Hit :type Hit%20Result%20Structure%20%28by%20ref%29))
  (if (not (Variables|Default|GetisMovingOnInit))
    (Utilities|Casting|CastToBP_PlayerPaw OtherActor)
    (Utilities|FlowControl|DoOnce false
      (:Completed
        (CallFunction|Tut)))))

(event OnComponentBeginOverlap(snowpile)
  (params (OverlappedComponent :type Primitive%20Component%20Object%20Reference) (OtherActor :type Actor%20Object%20Reference) (OtherComp :type Primitive%20Component%20Object%20Reference) (OtherBodyIndex :type Integer) (bFromSweep :type Boolean) (SweepResult :type Hit%20Result%20Structure%20%28by%20ref%29))
  (bind _asbp_player_paw (Utilities|Casting|CastToBP_PlayerPaw OtherActor))
  (Utilities|FlowControl|DoOnce false
    (:Completed
      (Class|PrimitiveComponent|SetAllPhysicsLinearVelocity (Variables|/Game/BluePrints/Player/BP_PlayerPaw.BP_PlayerPaw_C|GetCapsule _asbp_player_paw) "0, 0, 0" false)
      (Class|PrimitiveComponent|SetAllPhysicsAngularVelocityinDegrees (Variables|/Game/BluePrints/Player/BP_PlayerPaw.BP_PlayerPaw_C|GetCapsule _asbp_player_paw) (Math|Vector|MakeVector 0.0 0.0 0.0) false))))

(event Custom|CallSwitchPlatform
  (bind _movementspline (Variables|Default|GetMovementSpline))
  (Components|DestroyComponent (Variables|Default|GetRightWall))
  (Variables|Default|SetisStop true)
  (bind _alpha (Timeline|Timeline PlayFromStart)
    (:Update
      (Transformation|SetWorldLocation (Variables|Default|GetCube) (Spline|GetLocationatDistanceAlongSpline _movementspline (Math|Float|Lerp 0.0 (Spline|GetSplineLength _movementspline) _alpha) "World") false false))
    (:Finished
      (if (not (Variables|Default|GetisStop))
        (Utilities|FlowControl|FlipFlop
          (:A
            (if (Variables|Default|GetisMovingOnInit)
              (Timeline|Timeline PlayFromStart))))))))

(event Custom|tut
  (bind _movementspline (Variables|Default|GetMovementSpline))
  (bind _alpha (Timeline|Timeline PlayFromStart)
    (:Update
      (Transformation|SetWorldLocation (Variables|Default|GetCube) (Spline|GetLocationatDistanceAlongSpline _movementspline (Math|Float|Lerp 0.0 (Spline|GetSplineLength _movementspline) _alpha) "World") false false))
    (:Finished
      (if (not (Variables|Default|GetisStop))
        (Utilities|FlowControl|FlipFlop
          (:A
            (if (Variables|Default|GetisMovingOnInit)
              (Timeline|Timeline PlayFromStart))))))))

(event EventBeginPlay
  (bind _movementspline (Variables|Default|GetMovementSpline))
  (if (Variables|Default|GetisHasRightWall)
    _
    (else
      (Components|DestroyComponent (Variables|Default|GetRightWall))))
  (if (Variables|Default|GetisMovingOnInit)
    (Components|Timeline|SetPlayRate (Variables|Default|GetTimeline) (Variables|Default|GetmovingRate))
    (Utilities|FlowControl|FlipFlop :!label _label
      (:A
        (if (Variables|Default|GetisMovingOnInit)
          (bind _alpha (Timeline|Timeline PlayFromStart)
            (:Update
              (Transformation|SetWorldLocation (Variables|Default|GetCube) (Spline|GetLocationatDistanceAlongSpline _movementspline (Math|Float|Lerp 0.0 (Spline|GetSplineLength _movementspline) _alpha) "World") false false))
            (:Finished
              (if (not (Variables|Default|GetisStop))
                (goto _label)))))))))

(event Collision|EventActorBeginOverlap
  (params (OtherActor :type Actor%20Object%20Reference)))

(event EventTick
  (params (DeltaSeconds :type Float%20%28single-precision%29)))

(fn ConstructionScript)