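; GM_Stuck is the game mode that manages save and load of level, player transform and door states.
; BeginPlay reads GI_Stuck's slot name, then creates a BP_SaveGame or loads it, opening the saved map or restoring state.
; Dispatcher and retriever events sync Map_Main doors with a map keyed by GateNameString.
; Other events save at a given location, open Map_Main1, delete-and-restart, or record level changes without saved location.
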(event Custom|SaveDataRetriever
  (params (SaveRef :type BP%20Save%20Game%20Object%20Reference))
  (Utilities|IsValid SaveRef
    (:Is%20Valid
      (CallFunction|RetrieveGateOpenBoolean SaveRef))))

(event Custom|SaveDataDispacher
  (params (SaveRef :type BP%20Save%20Game%20Object%20Reference))
  (Utilities|IsValid SaveRef
    (:Is%20Valid
      (CallFunction|DispatchGateOpenBoolean SaveRef))))

(event Custom|RestartLevel
  ;[1 1 1] Delete save + Restart
  (SaveGame|DeleteGameinSlot (Variables|Default|GetSaveFileName))
  (Development|ExecuteConsoleCommand "RestartLevel" 0))

(event Custom|ChangeLevels
  (params (MapName :type Name))
  ;[1 1 1] change levels
  (bind _returnvalue (SaveGame|LoadGamefromSlot (Variables|Default|GetSaveFileName)))
  (bind _asbp_save_game (Utilities|Casting|CastToBP_SaveGame _returnvalue))
  (Variables|/Game/BluePrints/Saves/BP_SaveGame.BP_SaveGame_C|SetUseSavedLocation _asbp_save_game false)
  (Variables|/Game/BluePrints/Saves/BP_SaveGame.BP_SaveGame_C|SetMapName _asbp_save_game MapName)
  (SaveGame|SaveGametoSlot _asbp_save_game (Variables|Default|GetSaveFileName)))

(event Custom|save%20game
  (params (Location :type Vector))
  (bind _returnvalue (Game|Player|GetPlayerPawn 0))
  (bind _savefilename (Variables|Default|GetSaveFileName))
  (bind _asbp_player_paw (Utilities|Casting|CastToBP_PlayerPaw _returnvalue))
  (bind _capsule (Variables|/Game/BluePrints/Player/BP_PlayerPaw.BP_PlayerPaw_C|GetCapsule _asbp_player_paw))
  (bind _returnvalue_2 (Transformation|GetWorldTransform _capsule))
  ;[1 1 1] save game
  (bind _returnvalue_3 (SaveGame|LoadGamefromSlot (Variables|Default|GetSaveFileName)))
  (bind _asbp_save_game (Utilities|Casting|CastToBP_SaveGame _returnvalue_3))
  (Utilities|IsValid _asbp_player_paw
    (:Is%20Valid
      (Variables|/Game/BluePrints/Saves/BP_SaveGame.BP_SaveGame_C|SetPlayerTransform _asbp_save_game (Math|Transform|MakeTransform Location (.rotation _returnvalue_2) (.scale _returnvalue_2)))
      (Variables|/Game/BluePrints/Saves/BP_SaveGame.BP_SaveGame_C|SetUseSavedLocation _asbp_save_game true)
      (CallFunction|SaveDataRetriever _asbp_save_game)
      (SaveGame|SaveGametoSlot _asbp_save_game _savefilename)
      (Development|PrintString (Utilities|String|Append "Save game as " _savefilename) true true "(R=1.000000,G=0.330920,B=0.000000,A=1.000000)"))))

(event Custom|load%20game
  ;[1 1 1] load game
  (Game|OpenLevel(byName) "Map_Main1"))

(event Custom|DispatchPlayerTransform
  (params (SaveRef :type BP%20Save%20Game%20Object%20Reference))
  (bind _asbp_player_paw (Utilities|Casting|CastToBP_PlayerPaw (Game|Player|GetPlayerPawn 0)))
  (Development|PrintString "Hello")
  (Transformation|SetWorldTransform (Variables|/Game/BluePrints/Player/BP_PlayerPaw.BP_PlayerPaw_C|GetCapsule _asbp_player_paw) (Variables|/Game/BluePrints/Saves/BP_SaveGame.BP_SaveGame_C|GetPlayerTransform SaveRef) false false))

(event Custom|RetrieveGateOpenBoolean
  (params (SaveRef :type BP%20Save%20Game%20Object%20Reference))
  (bind _aregatesopen (Variables|/Game/BluePrints/Saves/BP_SaveGame.BP_SaveGame_C|GetareGatesOpen SaveRef))
  (bind _returnvalue (Game|GetCurrentLevelName true))
  (if (Utilities|Enum|Equal(Enum) _returnvalue "Map_Main")
    (bind _outactors (Actor|GetAllActorsOfClass "/Game/BluePrints/Immobiles/BP_SimpleMovingDoor.BP_SimpleMovingDoor_C"))
    (for _array_element _outactors
      (bind _keys (Utilities|Map|Keys _aregatesopen))
      (bind _array_element_2 (Utilities|Array|ForEachLoopwithBreak _keys :!label _label)
        (:LoopBody
          (if (Utilities|Enum|Equal(Enum) _array_element_2 (Variables|/Game/BluePrints/Immobiles/BP_SimpleMovingDoor.BP_SimpleMovingDoor_C|GetGateNameString _array_element))
            (Utilities|Map|Add _aregatesopen _array_element_2 (Variables|/Game/BluePrints/Immobiles/BP_SimpleMovingDoor.BP_SimpleMovingDoor_C|GetisOpen _array_element))
            (goto _label Break)))))))

(event Custom|DispatchGateOpenBoolean
  (params (SaveRef :type BP%20Save%20Game%20Object%20Reference))
  (bind _aregatesopen (Variables|/Game/BluePrints/Saves/BP_SaveGame.BP_SaveGame_C|GetareGatesOpen SaveRef))
  (bind _returnvalue (Game|GetCurrentLevelName true))
  (if (Utilities|Enum|Equal(Enum) _returnvalue "Map_Main")
    (bind _outactors (Actor|GetAllActorsOfClass "/Game/BluePrints/Immobiles/BP_SimpleMovingDoor.BP_SimpleMovingDoor_C"))
    (for _array_element _outactors
      (bind _keys (Utilities|Map|Keys _aregatesopen))
      (bind _array_element_2 (Utilities|Array|ForEachLoopwithBreak _keys :!label _label)
        (:LoopBody
          (if (Utilities|Enum|Equal(Enum) _array_element_2 (Variables|/Game/BluePrints/Immobiles/BP_SimpleMovingDoor.BP_SimpleMovingDoor_C|GetGateNameString _array_element))
            (bind _output_get (Variables|/Game/BluePrints/Immobiles/BP_SimpleMovingDoor.BP_SimpleMovingDoor_C|SetisOpen _array_element (.Value (Utilities|Map|Find _aregatesopen _array_element_2))))
            (if _output_get
              (Default|CallSwitchDoor _array_element)
              (goto _label Break)
              (else
                (goto _label Break)))))))))

(event EventBeginPlay
  (bind _asgi_stuck (Utilities|Casting|CastToGI_Stuck (Game|GetGameInstance)))
  (Variables|Default|SetSaveFileName (Variables|/Game/GI_Stuck.GI_Stuck_C|GetSaveFileName _asgi_stuck))
  (bind _returnvalue (SaveGame|DoesSaveGameExist (Variables|Default|GetSaveFileName)))
  (if _returnvalue
    (Development|PrintString "save file name exists")
    ;[1 1 1] load game
    (bind _returnvalue_2 (SaveGame|LoadGamefromSlot (Variables|Default|GetSaveFileName)))
    (bind _asbp_save_game (Utilities|Casting|CastToBP_SaveGame _returnvalue_2))
    (Variables|Default|SetSaveGameRef _asbp_save_game)
    (bind _returnvalue_3 (Game|GetCurrentLevelName true))
    (if (== _returnvalue_3 (Variables|/Game/BluePrints/Saves/BP_SaveGame.BP_SaveGame_C|GetMapName (Variables|Default|GetSaveGameRef)))
      (if (Variables|/Game/BluePrints/Saves/BP_SaveGame.BP_SaveGame_C|GetUseSavedLocation _asbp_save_game)
        ;[1 1 1] load game functionality
        (CallFunction|DispatchPlayerTransform _asbp_save_game))
      (CallFunction|SaveDataDispacher _asbp_save_game)
      (else
        (Game|OpenLevel(byName) (Variables|/Game/BluePrints/Saves/BP_SaveGame.BP_SaveGame_C|GetMapName (Variables|Default|GetSaveGameRef)))))
    (else
      ;[1 1 1] create save file
      (bind _returnvalue_4 (SaveGame|CreateSaveGameObject "/Game/BluePrints/Saves/BP_SaveGame.BP_SaveGame_C"))
      (bind _returnvalue_5 (Game|GetCurrentLevelName true))
      (Variables|/Game/BluePrints/Saves/BP_SaveGame.BP_SaveGame_C|SetMapName _returnvalue_4 (Utilities|String|StringToName _returnvalue_5))
      (CallFunction|SaveDataRetriever _returnvalue_4)
      (SaveGame|SaveGametoSlot _returnvalue_4 (Variables|Default|GetSaveFileName)))))

(event EventTick
  (params (DeltaSeconds :type Float%20%28single-precision%29)))

(fn ConstructionScript)